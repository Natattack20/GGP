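; Base town car actor that shuttles its Car component back and forth along local X in an endless ambient loop.
; BeginPlay caches the starting relative transform, then chained MoveComponentTo calls drive out by SingleDistance, rest, make a sideways-shifted half-turn, return, and repeat.
; Drive time scales with distance via SingleTurnTimeRate.
; Tick respawns two short-lived BP_CarExhaust actors at SpawnExhaust whenever both previous ones have expired.
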(event `self.ReceiveBeginPlay`
  ;[1 1 1] Comment
  (set `self.OriginTransForm` (`SceneComponent.GetRelativeTransform` (`self.Car`)))
  (`self.Move`))

(event `Move`
  (bind _car (`self.Car`))
  (bind _origintransform (`self.OriginTransForm`))
  (bind _origintransform_location (`KismetMathLibrary.BreakTransform` (`self.OriginTransForm`)))
  (bind _origintransform_2 (`self.OriginTransForm`))
  (bind (_origintransform_location_2 _origintransform_rotation) (`KismetMathLibrary.BreakTransform` (`self.OriginTransForm`)))
  (bind _resttime (`self.RestTime`))
  (bind _singledistance (`self.SingleDistance`))
  (bind _returnvalue (+ _origintransform_location_2 (`KismetMathLibrary.MakeVector` _singledistance)))
  (bind _returnvalue_2 (+ (.yaw (.rotation _origintransform)) 180.0))
  (bind _returnvalue_3 (* (`KismetMathLibrary.Abs` _singledistance) (`self.SingleTurnTimeRate`)))
  ;[1 1 1] Move
  (`KismetSystemLibrary.MoveComponentTo` _car _returnvalue _origintransform_rotation false false _returnvalue_3 :!label _label)
  (`KismetSystemLibrary.Delay` _resttime)
  (`KismetSystemLibrary.MoveComponentTo` _car (+ _returnvalue (0.0 150.0 0.0)) (`KismetMathLibrary.MakeRotator` (.roll (.rotation _origintransform)) (.pitch (.rotation _origintransform)) _returnvalue_2) false false 1.0)
  (`KismetSystemLibrary.MoveComponentTo` _car _origintransform_location (`KismetMathLibrary.MakeRotator` (.roll (.rotation _origintransform)) (.pitch (.rotation _origintransform)) _returnvalue_2) false false _returnvalue_3)
  (`KismetSystemLibrary.Delay` _resttime)
  (`KismetSystemLibrary.MoveComponentTo` _car (+ (.location _origintransform_2) (0.0 -150.0 0.0)) (`KismetMathLibrary.MakeRotator` (.roll (.rotation _origintransform_2)) (.pitch (.rotation _origintransform_2)) (.yaw (.rotation _origintransform_2))) false false 1.0)
  (goto _label))

(event `self.ReceiveTick`
  (params (DeltaSeconds :type "Float (single-precision)"))
  ;[1 1 1] Move
  (`/Engine/EditorBlueprintResources/StandardMacros.IsValid` (`self.Exhaust`)
    (:`Is Not Valid`
      (`/Engine/EditorBlueprintResources/StandardMacros.IsValid` (`self.Exhaust1`)
        (:`Is Not Valid`
          (`self.SpawnCarExhaust`))))))

(event `SpawnCarExhaust`
  ;[1 1 1] Move
  (bind _returnvalue (`|SpawnActorFromClass` "/Game/Chen/Blueprints/Xinyue/BP_CarExhaust.BP_CarExhaust_C" (`SceneComponent.K2_GetComponentToWorld` (`self.SpawnExhaust`)) "AlwaysSpawn" "MultiplyWithRoot" null null))
  (`self.SetLifeSpan` _returnvalue 1.5)
  (set `self.Exhaust` _returnvalue)
  (bind _returnvalue_2 (`|SpawnActorFromClass` "/Game/Chen/Blueprints/Xinyue/BP_CarExhaust.BP_CarExhaust_C" (`SceneComponent.K2_GetComponentToWorld` (`self.SpawnExhaust`)) "AlwaysSpawn" "MultiplyWithRoot" null null))
  (`self.SetLifeSpan` _returnvalue_2 1.5)
  (set `self.Exhaust1` _returnvalue_2))

(fn `UserConstructionScript`)