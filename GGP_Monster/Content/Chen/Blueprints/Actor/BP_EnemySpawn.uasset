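; BP_EnemySpawn is a trigger actor that spawns BP_UAVAI enemies when the third-person character enters its Box.
; The overlap fires only once through a DoOnce, then switches on SpawnNum to choose the SpawnPoint1 or SpawnPoint2 tag.
; It finds all actors with that tag and spawns one UAV at each of their transforms.
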(event `self.Box.OnComponentBeginOverlap`
  (params (OverlappedComponent :type "PrimitiveComponent Object Reference") (OtherActor :type "Actor Object Reference") (OtherComp :type "PrimitiveComponent Object Reference") (OtherBodyIndex :type Integer) (bFromSweep :type Boolean) (SweepResult :type "HitResult Structure (by ref)"))
  (cast `/Game/ThirdPerson/Blueprints/BP_ThirdPersonCharacter` OtherActor)
  (`/Engine/EditorBlueprintResources/StandardMacros.DoOnce` false
    (:`Completed`
      (switch `int` (`self.SpawnNum`)
        (:`0`
          (bind _outactors (`GameplayStatics.GetAllActorsWithTag` "SpawnPoint1"))
          (for _array_element _outactors
            (`|SpawnActorFromClass` "/Game/ZiyuanTest/BP_AIEnemy/Enemy/AI/BP_UAVAI.BP_UAVAI_C" (`self.GetTransform` _array_element) "Undefined" "MultiplyWithRoot" null null)))
        (:`1`
          (bind _outactors_2 (`GameplayStatics.GetAllActorsWithTag` "SpawnPoint2"))
          (for _array_element_2 _outactors_2
            (`|SpawnActorFromClass` "/Game/ZiyuanTest/BP_AIEnemy/Enemy/AI/BP_UAVAI.BP_UAVAI_C" (`self.GetTransform` _array_element_2) "Undefined" "MultiplyWithRoot" null null)))))))

(fn `UserConstructionScript`)