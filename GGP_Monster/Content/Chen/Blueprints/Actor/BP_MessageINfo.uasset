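; BP_MessageINfo is a world-space message actor that displays a key-info title through a WBP_KeyInfo widget component.
; On BeginPlay it passes InText to the widget as the title, then shifts itself vertically by a configurable local Z offset.
; Each Tick it turns yaw-only toward the player camera, acting as an upright billboard.
; A DestoryKeyInfo event destroys the actor.
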(event `self.ReceiveBeginPlay`
  (bind _aswbp_key_info (cast `/Game/Chen/Blueprints/Actor/WBP_KeyInfo` (`WidgetComponent.GetUserWidgetObject` (`self.Widget`))))
  (`/Game/Chen/Blueprints/Actor/WBP_KeyInfo.SetItemTitleName` _aswbp_key_info (`self.In Text`))
  (`self.K2_AddActorLocalOffset` (`KismetMathLibrary.MakeVector` 0.0 0.0 (`self.Delta Location Z`))))

(event `self.ReceiveTick`
  (params (DeltaSeconds :type "Float (single-precision)"))
  (bind (_returnvalue_roll _returnvalue_pitch _returnvalue_yaw) (`KismetMathLibrary.BreakRotator` (`KismetMathLibrary.FindLookAtRotation` (`SceneComponent.K2_GetComponentLocation` (`self.Widget`)) (`SceneComponent.K2_GetComponentLocation` (`Actor.RootComponent` (`GameplayStatics.GetPlayerCameraManager` 0))))))
  (`self.K2_SetActorRotation` (`KismetMathLibrary.MakeRotator` 0.0 0.0 _returnvalue_yaw)))

(event `DestoryKeyInfo`
  (`self.K2_DestroyActor`))

(fn `UserConstructionScript`)