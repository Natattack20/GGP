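; BP_Key is a key actor with a configurable static mesh, color and accompanying info message.
; On BeginPlay it spawns a BP_MessageINfo at the mesh location, passing its text and Z offset, and tears that message down on EndPlay.
; Helper functions swap the mesh and tint it through a dynamic instance of MI_KeyColor_Inst using the KeyColor parameter.
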(event `self.ReceiveBeginPlay`
  (bind _returnvalue (`|SpawnActorFromClass` "/Game/Chen/Blueprints/Actor/BP_MessageINfo.BP_MessageINfo_C" (`KismetMathLibrary.MakeTransform` (`SceneComponent.K2_GetComponentLocation` (`self.StaticMesh`))) "Undefined" "MultiplyWithRoot" null (`self.In Text`) (`self.Delta Location Z`) null))
  (set `self.KeyMessage` _returnvalue))

(event `self.ReceiveTick`
  (params (DeltaSeconds :type "Float (single-precision)")))

(event `self.ReceiveEndPlay`
  (params (EndPlayReason :type "EEndPlayReason Enum" :default "Destroyed"))
  (`/Game/Chen/Blueprints/Actor/BP_MessageINfo.DestoryKeyInfo` (`self.KeyMessage`)))

(fn `SetKeyStaticMeshColor`
  (params (Value :type "LinearColor Structure"))
  (bind _returnvalue (`KismetMaterialLibrary.CreateDynamicMaterialInstance` "/Game/Chen/Blueprints/Actor/MI_KeyColor_Inst.MI_KeyColor_Inst"))
  (`PrimitiveComponent.SetMaterial` (`self.StaticMesh`) 0 _returnvalue)
  (`MaterialInstanceDynamic.SetVectorParameterValue` _returnvalue "KeyColor" Value))

(fn `SetStaticMesh`
  (params (StaticMesh :type "StaticMesh Object Reference"))
  (`StaticMeshComponent.SetStaticMesh` (`self.StaticMesh`) StaticMesh))

(fn `UserConstructionScript`)