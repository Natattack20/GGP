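; Level 1 door trigger actor that opens the level's door when a person holds all the required items.
; CheckKeysID looks up each TiggerNum entry in the passed item map, stopping at the first failed check.
; On success, the Opendoor timeline drives the absolute Z location of the first BP_Level1Door found in the world, keeping X and Y.
; Both outcomes print a debug message.
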(event `CheckKeysID`
  (params (PersonItemMap :type "Map of Integer to String"))
  (for _array_element (`self.TiggerNum`)
    (if (`.ReturnValue` (`BlueprintMapLibrary.Map_Find` PersonItemMap _array_element))
      (set `self.isOpendoor?` true)
      (else
        (set `self.isOpendoor?` false)
        (break))))
  (if (`self.isOpendoor?`)
    (`KismetSystemLibrary.PrintString` "Opendoor")
    (bind _outactors (`GameplayStatics.GetAllActorsOfClass` "/Game/Chen/Blueprints/Actor/BP_Level1Door.BP_Level1Door_C"))
    (bind (_direction _newtrack_0) (`Timeline|Opendoor`)
      (:`Update`
        (bind _output (`|GetArrayItem` _outactors))
        (bind (_returnvalue_x _returnvalue_y) (`KismetMathLibrary.BreakVector` (`self.K2_GetActorLocation` _output)))
        (`self.K2_SetActorLocation` _output (`KismetMathLibrary.MakeVector` _returnvalue_x _returnvalue_y _newtrack_0) false false)))
    (else
      (`KismetSystemLibrary.PrintString` "Cant opendoor"))))

(fn `UserConstructionScript`)