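; Test chest actor that opens on E press and adds a weapon to the third-person character's inventory.
; BeginPlay reads the Fireball row from the Weapons data table to set the contents mesh and particle; the random roll always selects it.
; Box overlap toggles input and the prompt, though Access is set true on both enter and exit.
; A timeline animates the lid, then reveals the contents and grants the weapon.
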(event `self.ReceiveBeginPlay`
  (bind _returnvalue (`KismetMathLibrary.RandomIntegerInRange` 0))
  (if (== _returnvalue 0)
    (bind _returnvalue_2 (`|GetDataTableRow` "/Game/Sandeep/Projectiles/Weapons.Weapons" "Fireball")
      (:`then`
        (bind _output_get (set `self.Weapon Data` _returnvalue_2))
        (bind (_weaponname _damage _maxammo _currentammo _maxclip _currentclip _staticmesh _particleeffect) (break `/Game/Sandeep/Projectiles/WeaponData` _output_get))
        (`StaticMeshComponent.SetStaticMesh` (`self.Contents`) _staticmesh)
        (`ParticleSystemComponent.SetTemplate` (`self.Contents (Particle)`) _particleeffect)))
    (elif (== _returnvalue 1)
      _)))

(event `self.Box.OnComponentBeginOverlap`
  (params (OverlappedComponent :type "PrimitiveComponent Object Reference") (OtherActor :type "Actor Object Reference") (OtherComp :type "PrimitiveComponent Object Reference") (OtherBodyIndex :type Integer) (bFromSweep :type Boolean) (SweepResult :type "HitResult Structure (by ref)"))
  (cast `/Game/ThirdPerson/Blueprints/BP_ThirdPersonCharacter` OtherActor)
  (`self.EnableInput` (`GameplayStatics.GetPlayerController` 0))
  (set `self.Access` true)
  (`SceneComponent.SetVisibility` (`self.E to Open`) true false))

(event `self.Box.OnComponentEndOverlap`
  (params (OverlappedComponent :type "PrimitiveComponent Object Reference") (OtherActor :type "Actor Object Reference") (OtherComp :type "PrimitiveComponent Object Reference") (OtherBodyIndex :type Integer))
  (cast `/Game/ThirdPerson/Blueprints/BP_ThirdPersonCharacter` OtherActor)
  (`self.DisableInput` (`GameplayStatics.GetPlayerController` 0))
  (set `self.Access` true)
  (`SceneComponent.SetVisibility` (`self.E to Open`) false false))

(event `Key|E`
  (params (Key :type "Key Structure"))
  (:`Pressed`
    (if (`self.Access`)
      (if (not (`self.Opened`))
        (`|ExecutionSequence`
          (:`then_0`
            (bind (_direction _newtrack_0) (`Timeline|Opening` :!via `PlayFromStart`)
              (:`Update`
                (`SceneComponent.K2_SetRelativeLocationAndRotation` (`self.Top`) (`KismetMathLibrary.VLerp` (0.0 0.0 75.0) (-100.0 0.0 72.0) _newtrack_0) (`KismetMathLibrary.RLerp` (struct :`Yaw` 180.0) (struct :`Pitch` -140.0 :`Yaw` 180.0) _newtrack_0) false false))
              (:`Finished`
                (set `self.Opened` true)
                (`SceneComponent.SetVisibility` (`self.Contents`) true false)
                (`SceneComponent.SetVisibility` (`self.Contents (Particle)`) true false)
                (bind _asbp_third_person_character (cast `/Game/ThirdPerson/Blueprints/BP_ThirdPersonCharacter` (stale `self.Box.OnComponentBeginOverlap` OtherActor)))
                (`/Game/ThirdPerson/Blueprints/BP_ThirdPersonCharacter.Add WeaponToInventory` _asbp_third_person_character (stale `self.ReceiveBeginPlay` _output_get))))))))))

(fn `UserConstructionScript`)