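; Map-interaction bubble that carries the player along BubbleDirection when touched.
; Overlap snaps Box to the player's mesh, disables movement and sets CanYouFly, then restores walking and destroys the bubble near BubbleDuration's end; ending overlap also restores walking.
; Tick consumes that flag to apply a dynamic rainbow material and tween the player's root via MoveComponentTo.
; While the flag is false, Tick also destroys the bubble after half BubbleDuration, touched or not.
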(event `self.ReceiveBeginPlay`)

(event `self.ReceiveTick`
  (params (DeltaSeconds :type "Float (single-precision)"))
  (bind (_bubbledirection_x _bubbledirection_y _bubbledirection_z) (`KismetMathLibrary.BreakVector` (`self.BubbleDirection`)))
  (bind _rootcomponent (`Actor.RootComponent` (`GameplayStatics.GetPlayerCharacter` 0)))
  (bind (_returnvalue_x _returnvalue_y _returnvalue_z) (`KismetMathLibrary.BreakVector` (`SceneComponent.K2_GetComponentLocation` _rootcomponent)))
  ;[1 1 1] Move
  (if (`self.CanYouFly`)
    (bind _returnvalue (`PrimitiveComponent.CreateDynamicMaterialInstance` (`self.StaticMesh`) 0 "/Game/MapInteraction/Material/M_Bubble.M_Bubble" "None"))
    (bind _output_get (set `self.DynamicMaterial` _returnvalue))
    (`MaterialInstanceDynamic.SetVectorParameterValue` :`self` _output_get :`ParameterName` "RainbowRotator")
    (`MaterialInstanceDynamic.SetScalarParameterValue` _output_get "RainbowRotator" 5.0)
    (`KismetSystemLibrary.MoveComponentTo` _rootcomponent (`KismetMathLibrary.MakeVector` (+ _returnvalue_x _bubbledirection_x) (+ _returnvalue_y _bubbledirection_y) (+ _returnvalue_z _bubbledirection_z)) (`SceneComponent.K2_GetComponentRotation` _rootcomponent) false false (`self.BubbleDuration`))
    (set `self.CanYouFly` false)
    (else
      (`KismetSystemLibrary.Delay` (* (`self.BubbleDuration`) 0.5))
      (`self.K2_DestroyActor`))))

(event `self.StaticMesh.OnComponentBeginOverlap`
  (params (OverlappedComponent :type "PrimitiveComponent Object Reference") (OtherActor :type "Actor Object Reference") (OtherComp :type "PrimitiveComponent Object Reference") (OtherBodyIndex :type Integer) (bFromSweep :type Boolean) (SweepResult :type "HitResult Structure (by ref)"))
  (bind _returnvalue (`GameplayStatics.GetPlayerCharacter` 0))
  (bind _charactermovement (`Character.CharacterMovement` _returnvalue))
  ;[1 1 1] State
  (if (== OtherActor (`GameplayStatics.GetPlayerCharacter` 0))
    (`SceneComponent.K2_AttachToComponent` (`self.Box`) (`Character.Mesh` _returnvalue) "None" "SnapToTarget" "SnapToTarget" "KeepWorld" true)
    (`CharacterMovementComponent.SetMovementMode` _charactermovement "MOVE_None" 0)
    (set `self.CanYouFly` true)
    (`KismetSystemLibrary.Delay` (* (`self.BubbleDuration`) 0.8))
    (`CharacterMovementComponent.SetMovementMode` _charactermovement "MOVE_Walking" 0 :!pinned true) ; ReturnToMove
    (`KismetSystemLibrary.Delay` 0.2)
    (`ActorComponent.K2_DestroyComponent` (`self.Box`))
    (`self.K2_DestroyActor`)))

(event `self.StaticMesh.OnComponentEndOverlap`
  (params (OverlappedComponent :type "PrimitiveComponent Object Reference") (OtherActor :type "Actor Object Reference") (OtherComp :type "PrimitiveComponent Object Reference") (OtherBodyIndex :type Integer))
  (bind _returnvalue (`GameplayStatics.GetPlayerCharacter` 0))
  (if (== OtherActor _returnvalue)
    (`CharacterMovementComponent.SetMovementMode` (`Character.CharacterMovement` _returnvalue) "MOVE_Walking" 0 :!pinned true) ; ReturnToMove
  ))

(fn `UserConstructionScript`)