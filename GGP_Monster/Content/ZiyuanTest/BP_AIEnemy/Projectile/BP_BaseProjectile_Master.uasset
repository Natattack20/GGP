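; Base enemy projectile with configurable speed, gravity, trail, damage and impact effects, destroyed when its lifespan expires.
; On hit it detaches and stops the trail, hides the mesh and deactivates collision.
; A DoOnce limits impact handling to one hit: actors tagged Player get VFX, damage and a physics impulse if simulating.
; Anything else gets environment VFX and a fading decal actor aligned to the surface normal.
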(event `self.ReceiveBeginPlay`
  (bind _projectile_speed (`self.Projectile_Speed`))
  (bind _projectile (`self.Projectile`))
  (bind _projectile_particle_trails (`self.Projectile_Particle_Trails`))
  (`|ExecutionSequence`
    (:`then_0`
      ;[1 1 1 0.8] Spawn Trail
      (`/Engine/EditorBlueprintResources/StandardMacros.IsValid` _projectile_particle_trails
        (:`Is Valid`
          (bind _returnvalue (`NiagaraFunctionLibrary.SpawnSystemAttached` _projectile_particle_trails (`self.StaticMesh`) "None" (0.0 0.0 0.0) (struct) "KeepRelativeOffset" true)))))
    (:`then_1`
      (set `ProjectileMovementComponent.InitialSpeed` _projectile_speed _projectile)
      (set `ProjectileMovementComponent.MaxSpeed` _projectile_speed _projectile)
      (set `ProjectileMovementComponent.ProjectileGravityScale` (`self.Projectile_Gravity_Scale`) _projectile)
      (`KismetSystemLibrary.Delay` (`self.Projectile_LifeSpan`))
      (`self.K2_DestroyActor`))))

(event `self.ReceiveHit`
  (params (MyComp :type "PrimitiveComponent Object Reference") (Other :type "Actor Object Reference") (OtherComp :type "PrimitiveComponent Object Reference") (bSelfMoved :type Boolean) (HitLocation :type "Vector Structure") (HitNormal :type "Vector Structure") (NormalImpulse :type "Vector Structure") (Hit :type "HitResult Structure (by ref)"))
  (bind (_bblockinghit _binitialoverlap _time _distance _location _impactpoint _normal _impactnormal _physmat _hitactor _hitcomponent) (`GameplayStatics.BreakHitResult` Hit))
  (bind _hitlocation (`self.HitLocation`))
  (bind _returnvalue (`KismetMathLibrary.MakeRotFromX` (`self.HitNormal`)))
  (bind _returnvalue_2 (`KismetMathLibrary.SelectRotator` (`KismetMathLibrary.MakeRotFromX` (* (`self.GetActorForwardVector` self) -1.0)) _returnvalue (`self.UseHitNormal`)))
  (set `self.HitLocation` HitLocation)
  (set `self.HitNormal` HitNormal)
  (`|ExecutionSequence`
    (:`then_0`
      ;[1 1 1 0.8] Spawn Trail
      (`/Engine/EditorBlueprintResources/StandardMacros.IsValid` (`self.Projectile_Particle_Trails`)
        (:`Is Valid`
          (`SceneComponent.K2_DetachFromComponent` (stale `self.ReceiveBeginPlay` _returnvalue) "KeepWorld" "KeepWorld" "KeepWorld" true)
          (`FXSystemComponent.SetEmitterEnable` (stale `self.ReceiveBeginPlay` _returnvalue) "Trail" false))))
    (:`then_1`
      ;[1 1 1 0.8] Hide static mesh
      (`SceneComponent.SetVisibility` (`self.StaticMesh`) false false)
      (`ActorComponent.Deactivate` (`self.CollisionComponent`)))
    (:`then_2`
      ;[1 1 1 0.8] Spawn Hit VFX
      (`/Engine/EditorBlueprintResources/StandardMacros.DoOnce` false
        (:`Completed`
          (if (`self.ActorHasTag` _hitactor "Player")
            (`NiagaraFunctionLibrary.SpawnSystemAtLocation` (`self.Projectile_particle_When_Hit_Enemy`) _hitlocation _returnvalue_2 (1.0 1.0 1.0) true true "None" false)
            (`GameplayStatics.ApplyDamage` _hitactor (`self.Projectile_Damage`))
            (if (`SceneComponent.IsSimulatingPhysics` (`Actor.RootComponent` _hitactor) "None")
              (`PrimitiveComponent.AddImpulseAtLocation` _hitcomponent (* (`self.GetVelocity`) (`self.Projectile_ImpulseToPhysicsObject`)) (`self.K2_GetActorLocation`) "None"))
            (else
              (`NiagaraFunctionLibrary.SpawnSystemAtLocation` (`self.Projectile_particle_When_Hit_Environment`) _hitlocation _returnvalue_2)
              (`|SpawnActorFromClass` (`self.Projectile_Decal`) (`KismetMathLibrary.MakeTransform` (`self.HitLocation`) _returnvalue) "Undefined" "SelectDefaultAtRuntime" null (`self.Projectile_Decal_Material`) (`self.Projectile_Decal_FadeTime`) (`self.Projectile_Decal_Size_Multiplier`) null))))))))

(fn `UserConstructionScript`)