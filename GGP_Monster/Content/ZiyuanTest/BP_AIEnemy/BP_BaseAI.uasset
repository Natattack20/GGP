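; Base AI enemy Blueprint that keeps a shared count of living AI through an AICounter actor in the level.
; BeginPlay looks up the AICounter with GetActorOfClass and increments its Alive value.
; The BeDestroy event looks it up again and decrements Alive, with no caller for that event in this graph.
; Both events print the updated count to the screen.
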(event `self.ReceiveBeginPlay`
  (bind _returnvalue (`GameplayStatics.GetActorOfClass` "/Game/ZiyuanTest/BP_AIEnemy/AICounter.AICounter_C"))
  (bind _output_get (set `/Game/ZiyuanTest/BP_AIEnemy/AICounter.Alive` (+ (`/Game/ZiyuanTest/BP_AIEnemy/AICounter.Alive` _returnvalue) 1) _returnvalue))
  (`KismetSystemLibrary.PrintString` (`KismetStringLibrary.Conv_IntToString` _output_get)))

(event `BeDestroy`
  (bind _returnvalue (`GameplayStatics.GetActorOfClass` "/Game/ZiyuanTest/BP_AIEnemy/AICounter.AICounter_C"))
  (bind _output_get (set `/Game/ZiyuanTest/BP_AIEnemy/AICounter.Alive` (- (`/Game/ZiyuanTest/BP_AIEnemy/AICounter.Alive` _returnvalue) 1) _returnvalue))
  (`KismetSystemLibrary.PrintString` (`KismetStringLibrary.Conv_IntToString` _output_get)))

(fn `UserConstructionScript`)