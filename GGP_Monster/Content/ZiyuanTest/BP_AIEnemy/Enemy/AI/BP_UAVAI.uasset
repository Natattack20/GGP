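; Enemy UAV drone pawn that can roam around its spawn point, chase the player and fire projectile bursts.
; On BeginPlay it sets up its UAVControl blackboard and moves toward the player; Tick mirrors AIState to the blackboard, spins propellers and eases height to a fixed Z.
; ChasePlayer holds attack range, strafing and triggering randomized, muzzle-aimed bursts with a cooldown.
; FindRandomLocation and MoveAIToLocation provide radius-limited roaming with smoothed yaw.
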(event `RotatePropeller`
  (for _array_element (`|MakeArray` (`self.UAVP1`) (`self.UAVP2`) (`self.UAVP3`) (`self.UAVP4`))
    (`/Engine/EditorBlueprintResources/StandardMacros.IsValid` (`StaticMeshComponent.StaticMesh` _array_element)
      (:`Is Valid`
        (`SceneComponent.K2_AddLocalRotation` _array_element (`KismetMathLibrary.MakeRotator` 0.0 0.0 (* (`GameplayStatics.GetWorldDeltaSeconds`) 2000.0)) false false)))))

(event `self.ReceiveBeginPlay`
  (`parent.ReceiveBeginPlay`)
  (`|ExecutionSequence`
    (:`then_0`
      (bind _asuavcontrol (cast `/Game/ZiyuanTest/BP_AIEnemy/Enemy/UAVControl` (`self.GetController`)))
      (bind _output_get (set `self.As UAVControl` _asuavcontrol))
      (bind _blackboardcomponent (`AIController.UseBlackboard` _output_get "/Game/ZiyuanTest/BP_AIEnemy/Enemy/BB_UAVAI.BB_UAVAI"))
      (bind _output_get_2 (set `self.Blackboard Component` _blackboardcomponent))
      (`BlackboardComponent.SetValueAsObject` _output_get_2 "UAVActor" self))
    (:`then_1`
      (set `self.StartLocation` (`self.K2_GetActorLocation`)))
    (:`then_2`
      (bind _asbp_third_person_character (cast `/Game/Sandeep/BP_ThirdPersonCharacter` (`GameplayStatics.GetPlayerCharacter` 0)))
      (set `self.PlayerRef` _asbp_third_person_character))
    (:`then_3`
      (`|AIMoveTo` self (0.0 0.0 0.0) (`GameplayStatics.GetPlayerCharacter` 0) 1000.0))))

(event `ChaseStrafe`
  (bind _isa (`/Engine/EditorBlueprintResources/StandardMacros.FlipFlop`)
    (:`A`
      _)
    (:`B`
      _))
  (set `self.ChaseStrafeRight` _isa)
  (`KismetSystemLibrary.K2_SetTimerDelegate` (delegate `ChaseStrafe`)))

(event `CheckAndFire`
  (`/Game/ZiyuanTest/BP_AIEnemy/Enemy/ZiyuanMacros.ForLoopWithDelay` 1 (`KismetMathLibrary.RandomIntegerInRange` 3 (`self.BurstFireMax`)) (`self.WeaponRecoverTime`)
    (:`LoopBody`
      (`self.FindLookAtPlayer`)
      (if (`self.IsDead`)
        _
        (elif (not (`self.IsActorBeingDestroyed` (`GameplayStatics.GetPlayerCharacter` 0)))
          (`self.FireEffects`))))
    (:`Completed`
      (`KismetSystemLibrary.Delay` (`KismetMathLibrary.RandomFloatInRange` 2.5 4.5))
      (set `self.IsFiring` false))))

(event `self.ReceiveTick`
  (params (DeltaSeconds :type "Float (single-precision)"))
  (bind (_returnvalue_x _returnvalue_y) (`KismetMathLibrary.BreakVector` (`self.K2_GetActorLocation`)))
  (`|ExecutionSequence`
    (:`then_0`
      (`self.RotatePropeller`))
    (:`then_1`
      (`BlackboardComponent.SetValueAsEnum` (`self.Blackboard Component`) "UAVState" (`self.AIState`)))
    (:`then_2`
      (`self.K2_SetActorLocation` (`KismetMathLibrary.VLerp` (`self.K2_GetActorLocation`) (`KismetMathLibrary.MakeVector` _returnvalue_x _returnvalue_y 300.0) 0.2)))))

(event `FireEffects`
  (bind (_returnvalue_location _returnvalue_rotation) (`KismetMathLibrary.BreakTransform` (`SceneComponent.K2_GetComponentToWorld` (`self.Muzzle`))))
  (`|ExecutionSequence`
    (:`then_0`
      (`NiagaraFunctionLibrary.SpawnSystemAtLocation` "/Game/ZiyuanTest/VFX/Presets/Muzzle/NE_VFX_Muzzle_Energy_Burst_2.NE_VFX_Muzzle_Energy_Burst_2" _returnvalue_location _returnvalue_rotation)
      (`GameplayStatics.PlaySoundAtLocation` null _returnvalue_location (struct) 1.0 1.0 0.0 null null null null))
    (:`then_1`
      (`|SpawnActorFromClass` "/Game/ZiyuanTest/BP_AIEnemy/Projectile/BP_BaseProjectile_Master_Child.BP_BaseProjectile_Master_Child_C" (`SceneComponent.K2_GetComponentToWorld` (`self.Muzzle`)) "Undefined" "MultiplyWithRoot" null 100.0 0.0 1.0 50.0 1.0 null null null null 5.0 1.0 null))))

(fn `ChasePlayer`
  (returns (Return :type Boolean))
  (bind (_returnvalue_x _returnvalue_y _returnvalue_z) (`KismetMathLibrary.BreakVector` (`self.K2_GetActorLocation`)))
  (bind (_returnvalue_x_2 _returnvalue_y_2) (`KismetMathLibrary.BreakVector` (`self.K2_GetActorLocation` (`GameplayStatics.GetPlayerCharacter` 0))))
  (bind (_returnvalue_roll _returnvalue_pitch _returnvalue_yaw) (`KismetMathLibrary.BreakRotator` (`KismetMathLibrary.FindLookAtRotation` (`self.K2_GetActorLocation`) (`KismetMathLibrary.MakeVector` _returnvalue_x_2 _returnvalue_y_2 _returnvalue_z))))
  (bind _returnvalue (`KismetMathLibrary.Conv_RotatorToVector` (`KismetMathLibrary.MakeRotator` 0.0 0.0 _returnvalue_yaw)))
  (switch `/Game/ZiyuanTest/BP_AIEnemy/Enemy/Data/Chase_States` (`self.ChaseStates`)
    (:`NewEnumerator0`
      (if (> (`self.GetDistanceTo` (`GameplayStatics.GetPlayerCharacter` 0)) (`self.AttackDistance`))
        (`self.AddMovementInput` _returnvalue)
        (`self.K2_SetActorRotation` (`KismetMathLibrary.RLerp` (`self.K2_GetActorRotation`) (`KismetMathLibrary.MakeRotator` 0.0 0.0 _returnvalue_yaw) 0.1 true) :!label _label)
        (return false)
        (elif (< (`self.GetDistanceTo` (`GameplayStatics.GetPlayerCharacter` 0)) (- (`self.AttackDistance`) 100.0))
          (`self.AddMovementInput` _returnvalue -1.0)
          (goto _label)
          (else
            (`self.AddMovementInput` (`KismetMathLibrary.GetRightVector` (`KismetMathLibrary.FindLookAtRotation` (`self.K2_GetActorLocation`) (`self.K2_GetActorLocation` (`GameplayStatics.GetPlayerCharacter` 0)))) (`KismetMathLibrary.SelectFloat` -0.5 0.5 (`self.ChaseStrafeRight`)))
            (if (`self.IsFiring`)
              (goto _label)
              (else
                (set `self.IsFiring` true)
                (`self.CheckAndFire`)))))))))

(fn `FindLookAtPlayer`
  (`SceneComponent.K2_SetWorldRotation` (`self.Muzzle`) (`KismetMathLibrary.FindLookAtRotation` (`SceneComponent.K2_GetComponentLocation` (`self.Muzzle`)) (`self.K2_GetActorLocation` (`GameplayStatics.GetPlayerCharacter` 0))) false false))

(fn `FindRandomLocation`
  (returns (FinalTarget :type "Vector Structure"))
  (locals (Int :type Integer))
  (bind (_returnvalue_x _returnvalue_y _returnvalue_z) (`KismetMathLibrary.BreakVector` (`self.K2_GetActorLocation`)))
  (set `local.Int` 0)
  (set `self.TargetLocation` (`KismetMathLibrary.MakeVector` (+ _returnvalue_x (`KismetMathLibrary.RandomFloatInRange` -1000.0 1000.0)) (+ _returnvalue_y (`KismetMathLibrary.RandomFloatInRange` -1000.0 1000.0)) _returnvalue_z) :!label _label)
  (if (> (`KismetMathLibrary.Abs` (`KismetMathLibrary.VSize` (- (`self.StartLocation`) (`self.TargetLocation`)))) (`self.CanRoamRadius`))
    (bind _output_get (set `local.Int` (+ (`local.Int`) 1)))
    (if (< _output_get 10)
      (goto _label)
      (else
        (return (`self.StartLocation`))))
    (else
      (return (`self.TargetLocation`)))))

(fn `MoveAIToLocation`
  (params (MoveToLocation :type "Vector Structure") (Threshold :type "Float (double-precision)"))
  (returns (Complete :type Boolean))
  (bind (_returnvalue_x _returnvalue_y _returnvalue_z) (`KismetMathLibrary.BreakVector` (`self.K2_GetActorLocation`)))
  (bind (_returnvalue_roll _returnvalue_pitch _returnvalue_yaw) (`KismetMathLibrary.BreakRotator` (`KismetMathLibrary.FindLookAtRotation` (`self.K2_GetActorLocation`) (`KismetMathLibrary.MakeVector` (.x MoveToLocation) (.y MoveToLocation) _returnvalue_z))))
  (if (> (`KismetMathLibrary.VSize` (- (`self.K2_GetActorLocation`) MoveToLocation)) Threshold)
    (`self.AddMovementInput` (`KismetMathLibrary.Conv_RotatorToVector` (`KismetMathLibrary.MakeRotator` 0.0 0.0 _returnvalue_yaw)) 1.0 true)
    (`self.K2_SetActorRotation` (`KismetMathLibrary.RLerp` (`self.K2_GetActorRotation`) (`KismetMathLibrary.MakeRotator` 0.0 0.0 _returnvalue_yaw) 0.1 true))
    (return false)
    (else
      (return true))))

(fn `UserConstructionScript`
  (`parent.UserConstructionScript`))