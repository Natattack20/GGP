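; Self-destruct enemy that chases the player and explodes, damaging them if inside its Sphere and shaking the camera unless shielded.
; Box overlap starts material blinking and, with the player inside the Sphere, halts movement and charges a fuse that Tick detonates when full.
; Leaving early resets the fuse, while later exits leave it committed.
; A lifetime timer also blinks then detonates, and depleted health destroys it with a harmless explosion.
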(event `self.ReceiveBeginPlay`
  (bind _returnvalue (`GameplayStatics.GetPlayerCharacter` 0))
  (bind (_location _rotation) (`self.FaceToPlayer`))
  (bind (_location_2 _rotation_2) (`self.FaceToPlayer`))
  ;[1 1 1] Attack with Movement
  (`parent.ReceiveBeginPlay`)
  (`|ExecutionSequence`
    (:`then_0`
      (cast `/Game/ThirdPerson/Blueprints/BP_ThirdPersonCharacter` _returnvalue)
      (`self.FacePlayer`)
      (`KismetSystemLibrary.Delay` 1.0)
      (bind _asbp_third_person_character (cast `/Game/ThirdPerson/Blueprints/BP_ThirdPersonCharacter` _returnvalue :!label _label))
      (`|AIMoveTo` self (0.0 0.0 0.0) _asbp_third_person_character
        (:`then`
          (`KismetSystemLibrary.Delay` 0.1)
          (goto _label))))
    (:`then_1`
      (`KismetSystemLibrary.Delay` 15.0)
      (if (`PrimitiveComponent.IsOverlappingActor` (`self.Sphere`) (`GameplayStatics.GetPlayerCharacter` 0))
        (`GameplayStatics.SpawnEmitterAtLocation` "/Game/StarterContent/Particles/P_Explosion.P_Explosion" _location _rotation (2.5 2.5 2.5))
        (`GameplayStatics.ApplyDamage` (`GameplayStatics.GetPlayerCharacter` 0) 20.0)
        (`self.K2_DestroyActor`)
        (`self.BeDestroy`)
        (bind _returnvalue_2 (`GameplayStatics.GetActorOfClass` "/Game/ThirdPerson/Blueprints/BP_ThirdPersonCharacter.BP_ThirdPersonCharacter_C"))
        (if (not (`/Game/ThirdPerson/Blueprints/BP_ThirdPersonCharacter.Shield?` _returnvalue_2))
          (`GameplayStatics.PlayWorldCameraShake` "/Game/ZiyuanTest/BP_AIEnemy/BP_CameraShake.BP_CameraShake_C" (`self.K2_GetActorLocation`) 0.0 3000.0))
        (else
          (`GameplayStatics.SpawnEmitterAtLocation` "/Game/StarterContent/Particles/P_Explosion.P_Explosion" _location_2 _rotation_2 (2.5 2.5 2.5))
          (`self.K2_DestroyActor`)
          (`self.BeDestroy`))))
    (:`then_2`
      (`KismetSystemLibrary.Delay` 12.5)
      (`PrimitiveComponent.SetMaterial` (`self.Mesh`) 0 "/Engine/EngineDebugMaterials/TerrainCollisionMaterial.TerrainCollisionMaterial" :!label _label_2)
      (`KismetSystemLibrary.Delay` 0.3)
      (`PrimitiveComponent.SetMaterial` (`self.Mesh`) 0 "/Engine/BasicShapes/BasicShapeMaterial.BasicShapeMaterial")
      (`KismetSystemLibrary.Delay` 0.3)
      (goto _label_2))))

(event `self.ReceiveTick`
  (params (DeltaSeconds :type "Float (single-precision)"))
  (bind (_location _rotation) (`self.FaceToPlayer`))
  (bind (_location_2 _rotation_2) (`self.FaceToPlayer`))
  (bind _charactermovement (`self.CharacterMovement`))
  ;[1 1 1] Attack with Movement
  (`parent.ReceiveTick` DeltaSeconds)
  (`|ExecutionSequence`
    (:`then_0`
      (if (== (`self.Time`) 2.5)
        (if (`PrimitiveComponent.IsOverlappingActor` (`self.Sphere`) (`GameplayStatics.GetPlayerCharacter` 0))
          (`GameplayStatics.SpawnEmitterAtLocation` "/Game/StarterContent/Particles/P_Explosion.P_Explosion" _location _rotation (2.5 2.5 2.5))
          (`GameplayStatics.ApplyDamage` (`GameplayStatics.GetPlayerCharacter` 0) 20.0)
          (`self.K2_DestroyActor`)
          (`self.BeDestroy`)
          (bind _returnvalue (`GameplayStatics.GetActorOfClass` "/Game/ThirdPerson/Blueprints/BP_ThirdPersonCharacter.BP_ThirdPersonCharacter_C"))
          (if (not (`/Game/ThirdPerson/Blueprints/BP_ThirdPersonCharacter.Shield?` _returnvalue))
            (`GameplayStatics.PlayWorldCameraShake` "/Game/ZiyuanTest/BP_AIEnemy/BP_CameraShake.BP_CameraShake_C" (`self.K2_GetActorLocation`) 0.0 3000.0))
          (else
            (`GameplayStatics.SpawnEmitterAtLocation` "/Game/StarterContent/Particles/P_Explosion.P_Explosion" _location_2 _rotation_2 (2.5 2.5 2.5))
            (`self.K2_DestroyActor`)
            (`self.BeDestroy`)))))
    (:`then_1`
      (if (`self.Stop`)
        (`/Engine/EditorBlueprintResources/StandardMacros.DoOnce` false :!label _label_3
          (:`Completed`
            (`ActorComponent.SetActive` _charactermovement false false)
            (goto _label_4 :!via `Reset`)))
        (else
          (`/Engine/EditorBlueprintResources/StandardMacros.DoOnce` false :!label _label_4
            (:`Completed`
              (`ActorComponent.SetActive` _charactermovement true false)
              (goto _label_3 :!via `Reset`))))))))

(event `Move`
  ;[1 1 1] Attack with Movement
  ;;[1 1 1] Movement
  (bind _asbp_third_person_character (cast `/Game/ThirdPerson/Blueprints/BP_ThirdPersonCharacter` (`GameplayStatics.GetPlayerCharacter` 0)))
  (`|AIMoveTo` self (0.0 0.0 0.0) _asbp_third_person_character :!label _label_5
    (:`then`
      (if (not (`self.Stop`))
        (goto _label_5)))))

(event `FacePlayer`
  ;[1 1 1] Attack with Movement
  ;;[1 1 1] Movement
  (`self.K2_SetActorRotation` (`.Rotation` (`self.FaceToPlayer`)))
  (`KismetSystemLibrary.Delay` 0.001)
  (`self.FacePlayer`))

(event `self.Box.OnComponentBeginOverlap`
  (params (OverlappedComponent :type "PrimitiveComponent Object Reference") (OtherActor :type "Actor Object Reference") (OtherComp :type "PrimitiveComponent Object Reference") (OtherBodyIndex :type Integer) (bFromSweep :type Boolean) (SweepResult :type "HitResult Structure (by ref)"))
  ;[1 1 1] Timer
  (cast `/Game/ThirdPerson/Blueprints/BP_ThirdPersonCharacter` OtherActor)
  (`|ExecutionSequence`
    (:`then_0`
      (`/Engine/EditorBlueprintResources/StandardMacros.DoOnce` false :!label _label_6
        (:`Completed`
          (`PrimitiveComponent.SetMaterial` (`self.Mesh`) 0 "/Engine/EngineDebugMaterials/TerrainCollisionMaterial.TerrainCollisionMaterial" :!label _label_7)
          (`KismetSystemLibrary.Delay` 0.3)
          (`PrimitiveComponent.SetMaterial` (`self.Mesh`) 0 "/Engine/BasicShapes/BasicShapeMaterial.BasicShapeMaterial")
          (`KismetSystemLibrary.Delay` 0.3)
          (if (`self.Stop`)
            (goto _label_7)
            (else
              (goto _label_6 :!via `Reset`))))))
    (:`then_1`
      (if (`PrimitiveComponent.IsOverlappingActor` (`self.Sphere`) (`GameplayStatics.GetPlayerCharacter` 0))
        (set `self.Stop` true)
        (set `self.Time` (`KismetMathLibrary.FClamp` (+ (`self.Time`) 0.1) 0.0 2.5) :!label _label_8)
        (`KismetSystemLibrary.Delay` 0.1)
        (if (`PrimitiveComponent.IsOverlappingActor` (`self.Sphere`) (`GameplayStatics.GetPlayerCharacter` 0))
          (goto _label_8)
          (elif (>= (`self.Time`) 1.1)
            (goto _label_8)))))))

(event `self.Sphere.OnComponentEndOverlap`
  (params (OverlappedComponent :type "PrimitiveComponent Object Reference") (OtherActor :type "Actor Object Reference") (OtherComp :type "PrimitiveComponent Object Reference") (OtherBodyIndex :type Integer))
  ;[1 1 1] Timer
  (cast `/Game/ThirdPerson/Blueprints/BP_ThirdPersonCharacter` OtherActor)
  (if (<= (`self.Time`) 1.0)
    (set `self.Time` (`self.Retime`))
    (set `self.Stop` false)))

(event `self.ReceiveAnyDamage`
  (params (Damage :type "Float (single-precision)") (DamageType :type "DamageType Object Reference") (InstigatedBy :type "Controller Object Reference") (DamageCauser :type "Actor Object Reference"))
  (bind (_returnvalue_location _returnvalue_rotation) (`KismetMathLibrary.BreakTransform` (`self.GetTransform`)))
  ;[1 1 1] Health
  (bind _output_get (set `self.SDHealth` (`KismetMathLibrary.FClamp` (- (`self.SDHealth`) Damage) 0.0 100.0)))
  (if (<= _output_get 0.0)
    (`GameplayStatics.SpawnEmitterAtLocation` "/Game/StarterContent/Particles/P_Explosion.P_Explosion" _returnvalue_location _returnvalue_rotation)
    (`self.K2_DestroyActor`)))

(fn `UserConstructionScript`
  (`parent.UserConstructionScript`))