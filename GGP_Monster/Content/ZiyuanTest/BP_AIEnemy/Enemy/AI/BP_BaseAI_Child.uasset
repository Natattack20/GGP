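; Drone (UAV) enemy pawn that spins its four propellers each tick and provides helpers for roaming within a radius.
; On BeginPlay it registers itself in the UAVControl blackboard, records its start location and caches the player character.
; FindRandomLocation retries random nearby points, falling back to the start location after ten failures.
; MoveAIToLocation steers by movement input with lerped yaw at constant height, without pathfinding, and reports arrival.
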(event `RotatePropeller`
  (for _array_element (`|MakeArray` (`self.UAVP1`) (`self.UAVP2`) (`self.UAVP3`) (`self.UAVP4`))
    (`/Engine/EditorBlueprintResources/StandardMacros.IsValid` (`StaticMeshComponent.StaticMesh` _array_element)
      (:`Is Valid`
        (`SceneComponent.K2_AddLocalRotation` _array_element (`KismetMathLibrary.MakeRotator` 0.0 0.0 (* (`GameplayStatics.GetWorldDeltaSeconds`) 2000.0)) false false)))))

(event `self.ReceiveBeginPlay`
  (`parent.ReceiveBeginPlay`)
  (`|ExecutionSequence`
    (:`then_0`
      (bind _asuavcontrol (cast `/Game/ZiyuanTest/BP_AIEnemy/Enemy/UAVControl` (`self.GetController`)))
      (bind _output_get (set `self.As UAVControl` _asuavcontrol))
      (bind _blackboardcomponent (`AIController.UseBlackboard` _output_get null))
      (bind _output_get_2 (set `self.Blackboard Component` _blackboardcomponent))
      (`BlackboardComponent.SetValueAsObject` _output_get_2 "UAVActor" self))
    (:`then_1`
      (set `self.StartLocation` (`self.K2_GetActorLocation`)))
    (:`then_2`
      (bind _asbp_third_person_character (cast `/Game/Sandeep/BP_ThirdPersonCharacter` (`GameplayStatics.GetPlayerCharacter` 0)))
      (set `self.As BP Third Person Character` _asbp_third_person_character))))

(event `self.ReceiveTick`
  (params (DeltaSeconds :type "Float (single-precision)"))
  (`|ExecutionSequence`
    (:`then_0`
      (`self.RotatePropeller`))))

(fn `FindRandomLocation`
  (returns (FinalTarget :type "Vector Structure"))
  (locals (Int :type Integer))
  (bind (_returnvalue_x _returnvalue_y _returnvalue_z) (`KismetMathLibrary.BreakVector` (`self.K2_GetActorLocation`)))
  (set `local.Int` 0)
  (set `self.TargetLocation` (`KismetMathLibrary.MakeVector` (+ _returnvalue_x (`KismetMathLibrary.RandomFloatInRange` -1000.0 1000.0)) (+ _returnvalue_y (`KismetMathLibrary.RandomFloatInRange` -1000.0 1000.0)) _returnvalue_z) :!label _label)
  (if (> (`KismetMathLibrary.Abs` (`KismetMathLibrary.VSize` (- (`self.StartLocation`) (`self.TargetLocation`)))) (`self.CanRoamRadius`))
    (bind _output_get (set `local.Int` (+ (`local.Int`) 1)))
    (if (< _output_get 10)
      (goto _label)
      (else
        (return (`self.StartLocation`))))
    (else
      (return (`self.TargetLocation`)))))

(fn `MoveAIToLocation`
  (params (MoveToLocation :type "Vector Structure") (Threshold :type "Float (double-precision)"))
  (returns (Complete :type Boolean))
  (bind (_returnvalue_x _returnvalue_y _returnvalue_z) (`KismetMathLibrary.BreakVector` (`self.K2_GetActorLocation`)))
  (bind (_returnvalue_roll _returnvalue_pitch _returnvalue_yaw) (`KismetMathLibrary.BreakRotator` (`KismetMathLibrary.FindLookAtRotation` (`self.K2_GetActorLocation`) (`KismetMathLibrary.MakeVector` (.x MoveToLocation) (.y MoveToLocation) _returnvalue_z))))
  (if (> (`KismetMathLibrary.VSize` (- (`self.K2_GetActorLocation`) MoveToLocation)) Threshold)
    (`self.AddMovementInput` (`KismetMathLibrary.Conv_RotatorToVector` (`KismetMathLibrary.MakeRotator` 0.0 0.0 _returnvalue_yaw)) 1.0 true)
    (`self.K2_SetActorRotation` (`KismetMathLibrary.RLerp` (`self.K2_GetActorRotation`) (`KismetMathLibrary.MakeRotator` 0.0 0.0 _returnvalue_yaw) 0.2 true))
    (return false)
    (else
      (return true))))

(fn `UserConstructionScript`
  (`parent.UserConstructionScript`))