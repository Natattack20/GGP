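; Spawner_BP is a spawner actor that repeatedly spawns the configured EnemyType after random delays, starting on BeginPlay or through ActivateSpawner.
; It spawns at its own transform or at a random SpawnPoint_BP gathered at BeginPlay by matching ID.
; Each spawn plays a temporary heal-aura particle effect.
; The loop runs endlessly when Count is -1, otherwise counts down and destroys the spawner when finished.
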(event `self.ReceiveBeginPlay`
  (`|ExecutionSequence`
    (:`then_0`
      (if (`self.UseSpawnPoints`)
        (bind _outactors (`GameplayStatics.GetAllActorsOfClass` "/Game/ZiyuanTest/BP_SpawnerSystem/SpawnPoint_BP.SpawnPoint_BP_C"))
        (for _array_element _outactors
          (if (`KismetStringLibrary.EqualEqual_StrStr` (`/Game/ZiyuanTest/BP_SpawnerSystem/SpawnPoint_BP.SpawnPoint_ID` _array_element) (`self.SpawnPoints_ID`))
            (`KismetArrayLibrary.Array_AddUnique` (`self.SpawnPoints`) _array_element)))))
    (:`then_1`
      (if (`self.StartActive`)
        (`self.StartSpawning`)))))

(event `StartSpawning`
  (bind (_spawnlocation_location _spawnlocation_rotation _spawnlocation_scale) (`KismetMathLibrary.BreakTransform` (`self.SpawnLocation`)))
  (bind (_spawnlocation_location_2 _spawnlocation_rotation_2) (`KismetMathLibrary.BreakTransform` (`self.SpawnLocation`)))
  (`KismetSystemLibrary.Delay` (`KismetMathLibrary.RandomFloatInRange` (`self.SpawnDelay_Min`) (`self.SpawnDelay_Max`)) :!label _label)
  (if (`self.UseSpawnPoints`)
    (if (== (`KismetArrayLibrary.Array_Length` (`self.SpawnPoints`)) 1)
      (set `self.SpawnLocation` (`self.GetTransform` (`|GetArrayItem` (`self.SpawnPoints`))))
      (else
        (set `self.SpawnLocation` (`self.GetTransform` (`|GetArrayItem` (`self.SpawnPoints`) (`KismetMathLibrary.RandomIntegerInRange` 0 (- (`KismetArrayLibrary.Array_Length` (`self.SpawnPoints`)) 1)))))))
    (else
      (set `self.SpawnLocation` (`self.GetTransform`))))
  (`|SpawnActorFromClass` (`self.EnemyType`) (`KismetMathLibrary.MakeTransform` (+ _spawnlocation_location_2 (0.0 0.0 0.0)) _spawnlocation_rotation_2) "Undefined" "MultiplyWithRoot" null null)
  (bind _returnvalue (`GameplayStatics.SpawnEmitterAtLocation` "/Game/Sandeep/FXVarietyPack/Particles/P_ky_healAura.P_ky_healAura" _spawnlocation_location _spawnlocation_rotation _spawnlocation_scale))
  (`KismetSystemLibrary.Delay` 1.5)
  (`ActorComponent.K2_DestroyComponent` _returnvalue)
  (if (== (`self.Count`) -1)
    (goto _label)
    (else
      (set `self.Count` (- (`self.Count`) 1))
      (if (> (`self.Count`) 0)
        (goto _label)
        (else
          (`KismetSystemLibrary.Delay` 0.5)
          (`self.K2_DestroyActor`))))))

(event `ActivateSpawner`
  (`self.StartSpawning`))

(fn `UserConstructionScript`)