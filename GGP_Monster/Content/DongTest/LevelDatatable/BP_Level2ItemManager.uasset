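; Level 2 item manager that randomly places pickups when play begins.
; It reads every row of DT_Level2ItemInfo and handles only rows whose map name matches the current level.
; For each spawn count it picks a random location from the row's list, spawns the actor matching the item name, then removes that location to avoid reuse.
; Items include elemental pickups, DestroyBurst, shield frames, health packages and chests with a randomized type.
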(event `self.ReceiveBeginPlay`
  (bind _outrownames (`DataTableFunctionLibrary.GetDataTableRowNames` "/Game/DongTest/LevelDatatable/DT_Level2ItemInfo.DT_Level2ItemInfo"))
  (for _array_element _outrownames
    (bind _returnvalue (`|GetDataTableRow` "/Game/DongTest/LevelDatatable/DT_Level2ItemInfo.DT_Level2ItemInfo" _array_element)
      (:`then`
        (bind (_item_location _mapname _spawnnumber _itemname) (break `/Game/DongTest/LevelDatatable/BPS_ItemPoint` _returnvalue))
        (bind _output_get (set `self.Keylocation` _item_location))
        (bind _returnvalue_2 (`GameplayStatics.GetCurrentLevelName` true))
        (if (`KismetStringLibrary.EqualEqual_StrStr` _returnvalue_2 (`KismetStringLibrary.Conv_NameToString` _mapname))
          (for _ (range _spawnnumber)
            (if (not (<= (`KismetArrayLibrary.Array_Length` _output_get) 0))
              (bind _output_get_2 (set `self.RandomIndex` (`.OutIndex` (`KismetArrayLibrary.Array_Random` _output_get))))
              (`|ExecutionSequence`
                (:`then_0`
                  (if (== _itemname "Pitem_Fire")
                    (bind _returnvalue_3 (`KismetMathLibrary.MakeTransform` (`|GetArrayItem` (`self.Keylocation`) _output_get_2)))
                    (`|SpawnActorFromClass` "/Game/_Yifan/ItemSystem/_PassiveItems/BP_PItem_Fire_Sprite.BP_PItem_Fire_Sprite_C" _returnvalue_3 "Undefined" "MultiplyWithRoot" null null)
                    (`KismetArrayLibrary.Array_Remove` _output_get (`self.RandomIndex`) :!label _label)))
                (:`then_1`
                  (if (== _itemname "Pitem_Chill")
                    (`|SpawnActorFromClass` "/Game/_Yifan/ItemSystem/_PassiveItems/BP_PItem_Chill_Sprite.BP_PItem_Chill_Sprite_C" _returnvalue_3 "Undefined" "MultiplyWithRoot" null null)
                    (goto _label)))
                (:`then_2`
                  (if (== _itemname "DestroyBurst")
                    (`|SpawnActorFromClass` "/Game/_Yifan/ItemSystem/_ActiveItems/BP_DestroyBurst.BP_DestroyBurst_C" _returnvalue_3 "Undefined" "MultiplyWithRoot" null null)
                    (goto _label)))
                (:`then_3`
                  (if (== _itemname "Frame")
                    (`|SpawnActorFromClass` "/Game/_Yifan/ItemSystem/_ActiveItems/BP_FrameOfTheShield.BP_FrameOfTheShield_C" _returnvalue_3 "Undefined" "MultiplyWithRoot" null null)
                    (goto _label)))
                (:`then_4`
                  (if (== _itemname "Chest")
                    (bind _returnvalue_4 (`|SpawnActorFromClass` "/Game/Chest/BP_Chest.BP_Chest_C" _returnvalue_3 "Undefined" "MultiplyWithRoot" null null))
                    (set `/Game/Chest/BP_Chest.Integer for Type` (`KismetMathLibrary.RandomInteger` 2) _returnvalue_4)
                    (goto _label)))
                (:`then_5`
                  (if (== _itemname "HealthPackageted")
                    (`|SpawnActorFromClass` "/Game/_Yifan/ItemSystem/_PassiveItems/BP_PItem_HealthPackage.BP_PItem_HealthPackage_C" _returnvalue_3 "Undefined" "MultiplyWithRoot" null null)
                    (goto _label)))))))))))

(fn `UserConstructionScript`)