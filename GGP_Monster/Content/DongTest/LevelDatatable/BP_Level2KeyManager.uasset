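; BP_Level2KeyManager spawns key pickups for the current level when play begins, driven by the DT_Level2KeyInfo data table.
; Rows whose map name matches the current level each spawn a set number of BP_Key actors at randomly picked locations from that row.
; Each used location is removed from a working copy so keys do not share one, and every key receives its mesh, color, title, height offset, ID and name.
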(event `self.ReceiveBeginPlay`
  (bind _outrownames (`DataTableFunctionLibrary.GetDataTableRowNames` "/Game/DongTest/LevelDatatable/DT_Level2KeyInfo.DT_Level2KeyInfo"))
  (for _array_element _outrownames
    (bind _returnvalue (`|GetDataTableRow` "/Game/DongTest/LevelDatatable/DT_Level2KeyInfo.DT_Level2KeyInfo" _array_element)
      (:`then`
        (bind (_key_id _key_location _staticmesh _keycolor _iteamname _mapname _spawnnumber _titleinfo _offsidez) (break `/Game/Chen/Blueprints/Struct/BPS_SpawnPoint` _returnvalue))
        (bind _output_get (set `self.Keylocation` _key_location))
        (bind _returnvalue_2 (`GameplayStatics.GetCurrentLevelName` true))
        (if (`KismetStringLibrary.EqualEqual_StrStr` _returnvalue_2 (`KismetStringLibrary.Conv_NameToString` _mapname))
          (for _ (range _spawnnumber)
            (if (not (<= (`KismetArrayLibrary.Array_Length` _output_get) 0))
              (bind _output_get_2 (set `self.RandomIndex` (`.OutIndex` (`KismetArrayLibrary.Array_Random` _output_get))))
              (bind _returnvalue_3 (`|SpawnActorFromClass` "/Game/Chen/Blueprints/Actor/BP_Key.BP_Key_C" (`KismetMathLibrary.MakeTransform` (`|GetArrayItem` (`self.Keylocation`) _output_get_2)) "Undefined" "MultiplyWithRoot" null _titleinfo _offsidez null))
              (`KismetArrayLibrary.Array_Remove` _output_get (`self.RandomIndex`))
              (`/Game/Chen/Blueprints/Actor/BP_Key.SetStaticMesh` _returnvalue_3 _staticmesh)
              (`/Game/Chen/Blueprints/Actor/BP_Key.SetKeyStaticMeshColor` _returnvalue_3 (`KismetMathLibrary.Conv_ColorToLinearColor` _keycolor))
              (set `/Game/Chen/Blueprints/Actor/BP_Key.Item_ID` _key_id _returnvalue_3)
              (set `/Game/Chen/Blueprints/Actor/BP_Key.IteaName` _iteamname _returnvalue_3))))))))

(fn `UserConstructionScript`)