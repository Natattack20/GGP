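; BP_LabDoor is a proximity door that opens for the third-person character only while its Open flag is set.
; LevelOpen sets that flag, and Box overlap begin checks it before playing the DoorMovement timeline.
; Box overlap end reverses the timeline whatever the flag's state.
; The timeline animates the door by lerping its relative scale between OpenSize and CloseSize rather than moving it.
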(event `/Game/DongTest/LevelBP/BPI_LevelOpen.LevelOpen`
  (params (LevelOpen :type Boolean))
  (set `self.Open` LevelOpen))

(event `self.Box.OnComponentBeginOverlap`
  (params (OverlappedComponent :type "PrimitiveComponent Object Reference") (OtherActor :type "Actor Object Reference") (OtherComp :type "PrimitiveComponent Object Reference") (OtherBodyIndex :type Integer) (bFromSweep :type Boolean) (SweepResult :type "HitResult Structure (by ref)"))
  (cast `/Game/ThirdPerson/Blueprints/BP_ThirdPersonCharacter` OtherActor)
  (if (`self.Open`)
    (`self.DoorOpen`)))

(event `self.Box.OnComponentEndOverlap`
  (params (OverlappedComponent :type "PrimitiveComponent Object Reference") (OtherActor :type "Actor Object Reference") (OtherComp :type "PrimitiveComponent Object Reference") (OtherBodyIndex :type Integer))
  (cast `/Game/ThirdPerson/Blueprints/BP_ThirdPersonCharacter` OtherActor)
  (`self.DoorClose`))

(event `DoorOpen`
  (bind (_direction _lerpalpha) (`Timeline|DoorMovement` :!label _label)
    (:`Update`
      (`SceneComponent.SetRelativeScale3D` (`self.Door`) (`KismetMathLibrary.VLerp` (`self.OpenSize`) (`self.CloseSize`) _lerpalpha)))))

(event `DoorClose`
  (goto _label :!via `Reverse`))

(fn `UserConstructionScript`)