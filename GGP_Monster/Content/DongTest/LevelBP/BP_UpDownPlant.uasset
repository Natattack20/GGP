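; A moving platform (lift) that travels between an up and a down location when the third-person character enters its box trigger, once enabled through LevelOpen.
; Each trigger toggles direction, waits briefly, plays the Plant audio, flips the arrow and runs one of two timelines that lerp the root's world location.
; A Finish flag blocks retriggering until a delay started from the timeline update expires.
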(event `self.Box.OnComponentBeginOverlap`
  (params (OverlappedComponent :type "PrimitiveComponent Object Reference") (OtherActor :type "Actor Object Reference") (OtherComp :type "PrimitiveComponent Object Reference") (OtherBodyIndex :type Integer) (bFromSweep :type Boolean) (SweepResult :type "HitResult Structure (by ref)"))
  (bind _plant (`self.Plant`))
  (bind _defaultsceneroot (`self.DefaultSceneRoot`))
  (bind _details_arrow (`self.Details_Arrow`))
  (cast `/Game/ThirdPerson/Blueprints/BP_ThirdPersonCharacter` OtherActor)
  (if (`self.finish`)
    (if (`self.Open`)
      (set `self.UPorDown` (not (`self.UPorDown`)))
      (`KismetSystemLibrary.Delay` 0.5)
      (if (`self.UPorDown`)
        (`AudioComponent.Play` _plant 0.0)
        (`SceneComponent.K2_SetRelativeRotation` _details_arrow (struct :`Yaw` 180.0 :`Roll` -155.0) false false)
        (set `self.finish` false)
        (bind (_direction `_新建轨道_0`) (`Timeline|PlantUpDown` :!via `PlayFromStart`)
          (:`Update`
            (`SceneComponent.K2_SetWorldLocation` _defaultsceneroot (`KismetMathLibrary.VLerp` (`self.UpLocation`) (`self.DownLocation`) `_新建轨道_0`) false false)))
        (else
          (`AudioComponent.Play` _plant 0.0)
          (`SceneComponent.K2_SetRelativeRotation` _details_arrow (struct :`Roll` -25.0) false false)
          (set `self.finish` false)
          (bind (_direction_2 `_新建轨道_0_2`) (`Timeline|时间轴` :!via `PlayFromStart`)
            (:`Update`
              (`SceneComponent.K2_SetWorldLocation` _defaultsceneroot (`KismetMathLibrary.VLerp` (`self.DownLocation`) (`self.UpLocation`) `_新建轨道_0_2`) false false)))))
      (`KismetSystemLibrary.Delay` 4.0)
      (set `self.finish` true))))

(event `/Game/DongTest/LevelBP/BPI_LevelOpen.LevelOpen`
  (params (LevelOpen :type Boolean))
  (set `self.Open` LevelOpen))

(event `self.Plant.OnAudioFinished`
  (set `self.AudioFinish` true))

(fn `UserConstructionScript`)