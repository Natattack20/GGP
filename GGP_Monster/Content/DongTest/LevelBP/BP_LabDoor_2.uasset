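; Level 2 lab door that, once unlocked, opens when the player character enters its trigger box and closes on exit.
; The Level2DoorOpen event sets the Open flag, which gates opening and makes Tick tint the point light green.
; A timeline plays or reverses to lerp the door's relative scale, faking the movement.
; The door sound plays on enter and exit, guarded by a Finish flag so it never restarts mid-playback.
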(event `self.ReceiveTick`
  (params (DeltaSeconds :type "Float (single-precision)"))
  (if (`self.Open`)
    (`LightComponent.SetLightColor` (`self.PointLight`) (struct :`R` 0.246201 :`G` 1.0 :`B` 0.309469 :`A` 1.0) false)))

(event `/Game/DongTest/LevelBP/BPI_Level2Door.Level2DoorOpen`
  (params (DoorOpen :type Boolean))
  (set `self.Open` DoorOpen))

(event `self.Door1.OnAudioFinished`
  (set `self.Finish` true))

(event `self.Box.OnComponentBeginOverlap`
  (params (OverlappedComponent :type "PrimitiveComponent Object Reference") (OtherActor :type "Actor Object Reference") (OtherComp :type "PrimitiveComponent Object Reference") (OtherBodyIndex :type Integer) (bFromSweep :type Boolean) (SweepResult :type "HitResult Structure (by ref)"))
  (cast `/Game/ThirdPerson/Blueprints/BP_ThirdPersonCharacter` OtherActor)
  (if (`self.Open`)
    (`self.DoorOpen`)
    (if (`self.Finish`) :!label _label
      (`AudioComponent.Play` (`self.Door1`) 0.0)
      (set `self.Finish` false))))

(event `self.Box.OnComponentEndOverlap`
  (params (OverlappedComponent :type "PrimitiveComponent Object Reference") (OtherActor :type "Actor Object Reference") (OtherComp :type "PrimitiveComponent Object Reference") (OtherBodyIndex :type Integer))
  (cast `/Game/ThirdPerson/Blueprints/BP_ThirdPersonCharacter` OtherActor)
  (`self.DoorClose`)
  (goto _label))

(event `DoorOpen`
  (bind (_direction _lerpalpha) (`Timeline|DoorMovement` :!label _label_2)
    (:`Update`
      (`SceneComponent.SetRelativeScale3D` (`self.Door`) (`KismetMathLibrary.VLerp` (`self.OpenSize`) (`self.CloseSize`) _lerpalpha)))))

(event `DoorClose`
  (goto _label_2 :!via `Reverse`))

(fn `UserConstructionScript`)