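; BP_Jump2 is a one-shot triggered level actor that reveals a piece of itself and rises when the player character touches it.
; The first Box overlap by BP_ThirdPersonCharacter passes a DoOnce, stores the actor's location and makes Cube2 visible.
; A timeline then lerps the root component 750 units straight up from that stored location, without sweep.
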(event `self.Box.OnComponentBeginOverlap`
  (params (OverlappedComponent :type "PrimitiveComponent Object Reference") (OtherActor :type "Actor Object Reference") (OtherComp :type "PrimitiveComponent Object Reference") (OtherBodyIndex :type Integer) (bFromSweep :type Boolean) (SweepResult :type "HitResult Structure (by ref)"))
  (bind (_currentlocation_x _currentlocation_y _currentlocation_z) (`KismetMathLibrary.BreakVector` (`self.CurrentLocation`)))
  (cast `/Game/ThirdPerson/Blueprints/BP_ThirdPersonCharacter` OtherActor)
  (`/Engine/EditorBlueprintResources/StandardMacros.DoOnce` false
    (:`Completed`
      (set `self.CurrentLocation` (`self.K2_GetActorLocation`))
      (`SceneComponent.SetVisibility` (`self.Cube2`) true true)
      (bind (_direction _lerpalpha) (`Timeline|时间轴`)
        (:`Update`
          (`SceneComponent.K2_SetWorldLocation` (`self.DefaultSceneRoot`) (`KismetMathLibrary.VLerp` (`self.CurrentLocation`) (`KismetMathLibrary.MakeVector` _currentlocation_x _currentlocation_y (+ _currentlocation_z 750.0)) _lerpalpha) false false))))))

(fn `UserConstructionScript`)