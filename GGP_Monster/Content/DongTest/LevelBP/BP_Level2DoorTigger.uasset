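; Level 2 door trigger Blueprint that decides whether a door opens based on the items in a person's item map.
; CheckKeysID looks up every TiggerNum entry in the passed map, stopping at the first one missing.
; When all are found it sets IsOpendoor and only prints "Open".
; An Opendoor timeline meant to drive the actor's Z location is never triggered.
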(event `CheckKeysID`
  (params (PersonItemMap :type "Map of Integer to String"))
  (for _array_element (`self.TiggerNum`)
    (if (`.ReturnValue` (`BlueprintMapLibrary.Map_Find` PersonItemMap _array_element))
      (set `self.isOpendoor?` true)
      (else
        (set `self.isOpendoor?` false)
        (break))))
  (if (`self.isOpendoor?`)
    (`KismetSystemLibrary.PrintString` "Open")))

(fn `UserConstructionScript`)