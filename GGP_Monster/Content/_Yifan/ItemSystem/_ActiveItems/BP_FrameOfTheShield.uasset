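; Active item "Frame of the Shield" that grants the player a temporary shield with a fading visual effect.
; On activation it sets the character's Shield flag, attaches to the player mesh and reveals its hidden static mesh with a dynamic material.
; A timeline drives the material's Subtract parameter as the shield runs, then clears the flag and destroys the actor after a short delay.
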(event `self.ReceiveBeginPlay`
  (`parent.ReceiveBeginPlay`)
  (`SceneComponent.SetVisibility` (`self.StaticMesh`) false false))

(event `self.Activate Active Item`
  (`parent.Activate Active Item`)
  (bind _asbp_third_person_character (cast `/Game/ThirdPerson/Blueprints/BP_ThirdPersonCharacter` (`GameplayStatics.GetPlayerCharacter` 0)))
  (`|ExecutionSequence`
    (:`then_0`
      (set `/Game/ThirdPerson/Blueprints/BP_ThirdPersonCharacter.Shield?` true _asbp_third_person_character))
    (:`then_1`
      (`SceneComponent.K2_AttachToComponent` (`self.StaticMesh1`) (`Character.Mesh` _asbp_third_person_character) "None" "SnapToTarget" "SnapToTarget" "KeepWorld" true)
      (`SceneComponent.SetVisibility` (`self.StaticMesh`) true false)
      (bind _returnvalue (`PrimitiveComponent.CreateDynamicMaterialInstance` (`self.StaticMesh`) 0 "/Game/_Yifan/ItemSystem/Material_Item/M_FrameOfTheShield.M_FrameOfTheShield" "None"))
      (bind _output_get (set `self.DynamicMaterial` _returnvalue))
      (`MaterialInstanceDynamic.SetVectorParameterValue` :`self` _output_get :`ParameterName` "Subtract")
      (bind (_direction _lightgone) (`Timeline|Timeline` :!pinned true :!via `PlayFromStart`) ; SwitchTheShieldTimeAnd Frame_12s
        (:`Update`
          (`MaterialInstanceDynamic.SetScalarParameterValue` (`self.DynamicMaterial`) "Subtract" _lightgone))
        (:`Finished`
          (`|ExecutionSequence`
            (:`then_0`
              (bind _asbp_third_person_character_2 (cast `/Game/ThirdPerson/Blueprints/BP_ThirdPersonCharacter` (`GameplayStatics.GetPlayerCharacter` 0)))
              (set `/Game/ThirdPerson/Blueprints/BP_ThirdPersonCharacter.Shield?` false _asbp_third_person_character_2))
            (:`then_1`
              (`/Engine/EditorBlueprintResources/StandardMacros.IsValid` (`self.DefaultSceneRoot`)
                (:`Is Valid`
                  (`KismetSystemLibrary.Delay` 0.2)
                  (`self.K2_DestroyActor`))))))))))

(fn `UserConstructionScript`
  (`parent.UserConstructionScript`))