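; BP_DestroyBurst is an active item that sets off a lethal area explosion against AI enemies.
; On activation, a timeline grows the visible ExplodeArea and Box from zero scale while a recharge sound plays.
; When it finishes, it enables collision and Box physics, plays explosion sound and camera shake, flickers materials via delays, then destroys itself.
; ExplodeArea begin-overlaps deal massive damage to any BP_BaseAI.
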(event `self.Activate Active Item`
  (`parent.Activate Active Item`)
  (`KismetSystemLibrary.PrintString` "DestroyBurst Actived")
  (`SceneComponent.SetVisibility` (`self.ExplodeArea`) true false)
  (`GameplayStatics.PlaySoundAtLocation` "/Game/_Yifan/ItemSystem/Audios/DestroyBurst/Recharge_Energy_or_Skill_UI_Sound_8.Recharge_Energy_or_Skill_UI_Sound_8" (`self.K2_GetActorLocation`) (struct) 1.0 1.0 0.0 null null null null)
  ;[1 0.9242 0.5017 1 20] Scale in 1s
  (bind (_direction _scaletrack) (`Timeline|ScaleTimeline`)
    (:`Update`
      (bind _returnvalue (`KismetMathLibrary.VLerp` (0.0 0.0 0.0) (2.0 2.0 2.0) _scaletrack))
      (`SceneComponent.SetWorldScale3D` (`self.ExplodeArea`) _returnvalue)
      (`SceneComponent.SetWorldScale3D` (`self.Box`) _returnvalue))
    (:`Finished`
      (`PrimitiveComponent.SetMaterial` (`self.ExplodeArea`) 0 "/Game/_Yifan/ItemSystem/Material_Item/DestoryBurstFrame_Ready1.DestoryBurstFrame_Ready1")
      (`PrimitiveComponent.SetCollisionEnabled` (`self.ExplodeArea`) "QueryAndPhysics")
      (`PrimitiveComponent.SetCollisionEnabled` (`self.Box`) "QueryAndPhysics")
      (`PrimitiveComponent.SetSimulatePhysics` (`self.Box`) true)
      (`PrimitiveComponent.SetCollisionResponseToAllChannels` (`self.ExplodeArea`) "ECR_Overlap")
      (`GameplayStatics.PlaySoundAtLocation` "/Game/_Yifan/ItemSystem/Audios/DestroyBurst/Playful_Game_Explosion.Playful_Game_Explosion" (`self.K2_GetActorLocation`) (struct) 1.0 1.0 0.0 null null null null)
      (`GameplayStatics.PlayWorldCameraShake` "/Game/ZiyuanTest/BP_AIEnemy/BP_CameraShake.BP_CameraShake_C" (`self.K2_GetActorLocation`) 0.0 5000.0)
      (`KismetSystemLibrary.Delay` 0.05)
      (`PrimitiveComponent.SetMaterial` (`self.ExplodeArea`) 0 "/Game/_Yifan/ItemSystem/Material_Item/DestoryBurstFrame_Ready2.DestoryBurstFrame_Ready2")
      (`KismetSystemLibrary.Delay` 0.05)
      (`PrimitiveComponent.SetMaterial` (`self.ExplodeArea`) 0 "/Game/_Yifan/ItemSystem/Material_Item/DestoryBurstFrame_Ready1.DestoryBurstFrame_Ready1")
      (`KismetSystemLibrary.Delay` 0.05)
      (`PrimitiveComponent.SetMaterial` (`self.ExplodeArea`) 0 "/Game/_Yifan/ItemSystem/Material_Item/DestoryBurstFrame_Ready2.DestoryBurstFrame_Ready2")
      (`KismetSystemLibrary.Delay` 0.05)
      (`PrimitiveComponent.SetMaterial` (`self.ExplodeArea`) 0 "/Game/_Yifan/ItemSystem/Material_Item/DestoryBurstFrame_Ready1.DestoryBurstFrame_Ready1")
      (`KismetSystemLibrary.Delay` 0.3)
      (`self.K2_DestroyActor`))))

(event `self.ExplodeArea.OnComponentBeginOverlap`
  (params (OverlappedComponent :type "PrimitiveComponent Object Reference") (OtherActor :type "Actor Object Reference") (OtherComp :type "PrimitiveComponent Object Reference") (OtherBodyIndex :type Integer) (bFromSweep :type Boolean) (SweepResult :type "HitResult Structure (by ref)"))
  (bind _asbp_base_ai (cast `/Game/ZiyuanTest/BP_AIEnemy/BP_BaseAI` OtherActor))
  (`GameplayStatics.ApplyDamage` _asbp_base_ai 9999.0))

(event `self.ExplodeArea.OnComponentEndOverlap`
  (params (OverlappedComponent :type "PrimitiveComponent Object Reference") (OtherActor :type "Actor Object Reference") (OtherComp :type "PrimitiveComponent Object Reference") (OtherBodyIndex :type Integer)))

(fn `UserConstructionScript`
  (`parent.UserConstructionScript`))