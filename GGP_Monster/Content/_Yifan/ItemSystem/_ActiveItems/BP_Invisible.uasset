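; Active item that temporarily cloaks the player's third-person character.
; On activation it sets the character's Cloaking flag and swaps the Mesh and Cube materials to an invisible one.
; A looping one-second Delay decrements a clamped Timecount, which this graph never resets.
; At zero it clears the flag and applies a hardcoded WorldGridMaterial to both components instead of restoring their original materials.
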(event `self.Activate Active Item`
  (`parent.Activate Active Item`)
  (bind _asbp_third_person_character (cast `/Game/ThirdPerson/Blueprints/BP_ThirdPersonCharacter` (`GameplayStatics.GetPlayerCharacter` 0)))
  (set `/Game/ThirdPerson/Blueprints/BP_ThirdPersonCharacter.Cloaking?` true _asbp_third_person_character)
  (`PrimitiveComponent.SetMaterial` (`Character.Mesh` _asbp_third_person_character) 0 "/Game/ThirdPerson/Blueprints/Invsible.Invsible")
  (`PrimitiveComponent.SetMaterial` (`/Game/ThirdPerson/Blueprints/BP_ThirdPersonCharacter.Cube` _asbp_third_person_character) 0 "/Game/ThirdPerson/Blueprints/Invsible.Invsible")
  (set `self.Timecount` (`KismetMathLibrary.FClamp` (- (`self.Timecount`) 1.0) 0.0 20.0) :!label _label)
  (`KismetSystemLibrary.Delay` 1.0)
  (if (<= (`self.Timecount`) 0.0)
    (set `/Game/ThirdPerson/Blueprints/BP_ThirdPersonCharacter.Cloaking?` false _asbp_third_person_character)
    (`PrimitiveComponent.SetMaterial` (`/Game/ThirdPerson/Blueprints/BP_ThirdPersonCharacter.Cube` _asbp_third_person_character) 0 "/Engine/EngineMaterials/WorldGridMaterial.WorldGridMaterial")
    (`PrimitiveComponent.SetMaterial` (`Character.Mesh` _asbp_third_person_character) 0 "/Engine/EngineMaterials/WorldGridMaterial.WorldGridMaterial")
    (else
      (goto _label))))

(fn `UserConstructionScript`
  (`parent.UserConstructionScript`))