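; Passive item that grants or upgrades the third-person player character's jetpack.
; When its passive effect updates, it enables the jetpack and prints a debug message if the character has none.
; Otherwise it compounds a boost to maximum power and a cut to maximum cooldown, and clears the current cooldown.
; The power refill applies the multiplier again, leaving current power above the new maximum.
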(event `self.UpdatePassiveEffect`
  (`parent.UpdatePassiveEffect`)
  (bind _asbp_third_person_character (cast `/Game/ThirdPerson/Blueprints/BP_ThirdPersonCharacter` (`GameplayStatics.GetPlayerCharacter` 0)))
  (if (`/Game/ThirdPerson/Blueprints/BP_ThirdPersonCharacter.HasRpack` _asbp_third_person_character)
    (bind _returnvalue (* (`/Game/ThirdPerson/Blueprints/BP_ThirdPersonCharacter.MaxRpackPower` _asbp_third_person_character) 1.05))
    (set `/Game/ThirdPerson/Blueprints/BP_ThirdPersonCharacter.MaxRpackPower` _returnvalue _asbp_third_person_character)
    (set `/Game/ThirdPerson/Blueprints/BP_ThirdPersonCharacter.CurrentRpackPower` _returnvalue _asbp_third_person_character)
    (set `/Game/ThirdPerson/Blueprints/BP_ThirdPersonCharacter.RpackCoolDownMax` (* (`/Game/ThirdPerson/Blueprints/BP_ThirdPersonCharacter.RpackCoolDownMax` _asbp_third_person_character) 0.8) _asbp_third_person_character)
    (set `/Game/ThirdPerson/Blueprints/BP_ThirdPersonCharacter.RpackCoolDown` 0.0 _asbp_third_person_character)
    (else
      (set `/Game/ThirdPerson/Blueprints/BP_ThirdPersonCharacter.HasRpack` true _asbp_third_person_character)
      (`KismetSystemLibrary.PrintString` "--Jetpack Enabled--" true true (struct :`R` 1.0 :`B` 0.977855 :`A` 1.0)))))

(fn `UserConstructionScript`
  (`parent.UserConstructionScript`))