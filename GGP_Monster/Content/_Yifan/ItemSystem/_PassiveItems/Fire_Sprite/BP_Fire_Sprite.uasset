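; Fire Sprite passive-item actor that automatically shoots projectiles at the nearest enemy.
; A replaying timeline lerps the spring arm's world rotation toward a newly randomized pitch on each cycle.
; A looping timer scans all BP_BaseAI actors for the one closest to the sprite's mesh, then spawns BP_Fire_Sprite_Projectile toward it.
; Aim leads the target by simply adding its velocity to its location, without scaling for distance or projectile speed.
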(event `self.ReceiveBeginPlay`
  (bind _returnvalue (`KismetMathLibrary.RandomFloatInRange` -10.0 10.0))
  (`|ExecutionSequence`
    (:`then_0`
      (set `self.Random Pitch` _returnvalue)
      (bind (_direction _yaw) (`Timeline|Timeline` :!via `PlayFromStart` :!label _label)
        (:`Update`
          (`SceneComponent.K2_SetWorldRotation` (`self.SpringArm`) (`KismetMathLibrary.RLerp` (`SceneComponent.K2_GetComponentRotation` (`self.SpringArm`)) (`KismetMathLibrary.MakeRotator` 0.0 (`self.Random Pitch`)) _yaw) false false))
        (:`Finished`
          (set `self.Random Pitch` _returnvalue)
          (goto _label :!via `PlayFromStart`))))
    (:`then_1`
      (`KismetSystemLibrary.K2_SetTimerDelegate` (delegate `Attack Enemy`) 2.0 true))))

(event `Attack Enemy`
  ;[1 1 1] Finds the closest enemy
  (bind _outactors (`GameplayStatics.GetAllActorsOfClass` "/Game/ZiyuanTest/BP_AIEnemy/BP_BaseAI.BP_BaseAI_C"))
  (for (_array_element _array_index) _outactors
    (if (== _array_index 0)
      (bind _returnvalue (`KismetMathLibrary.Vector_Distance` (`SceneComponent.K2_GetComponentLocation` (`Character.CapsuleComponent` _array_element)) (`SceneComponent.K2_GetComponentLocation` (`self.StaticMesh`))))
      (bind _output_get (set `self.Distance` _returnvalue))
      (set `self.Closest Enemy` _array_element)
      (elif (< _returnvalue _output_get)
        (set `self.Distance` _returnvalue)
        (set `self.Closest Enemy` _array_element))))
  (`self.Fire Projectile`))

(event `Fire Projectile`
  (bind _closest_enemy (`self.Closest Enemy`))
  (bind _returnvalue (`SceneComponent.K2_GetComponentLocation` (`self.StaticMesh`)))
  ;[1 1 1] Smart Aim for the Fire Sprite
  (`|SpawnActorFromClass` "/Game/_Yifan/ItemSystem/_PassiveItems/Fire_Sprite/BP_Fire_Sprite_Projectile.BP_Fire_Sprite_Projectile_C" (`KismetMathLibrary.MakeTransform` _returnvalue (`KismetMathLibrary.FindLookAtRotation` _returnvalue (+ (`SceneComponent.K2_GetComponentLocation` (`Character.CapsuleComponent` _closest_enemy)) (`self.GetVelocity` _closest_enemy)))) "Undefined" "MultiplyWithRoot" null 5000.0 0.0 null false null))

(fn `UserConstructionScript`)