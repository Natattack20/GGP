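; Passive item Blueprint for a max health potion that raises the player character's maximum health.
; It overrides UpdatePassiveEffect, calls the parent, then casts player 0's character to BP_ThirdPersonCharacter and adds a fixed amount to MaxHealth.
; The increase is cumulative on each call and leaves current health untouched in this Blueprint.
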(event `self.UpdatePassiveEffect`
  (`parent.UpdatePassiveEffect`)
  (bind _asbp_third_person_character (cast `/Game/ThirdPerson/Blueprints/BP_ThirdPersonCharacter` (`GameplayStatics.GetPlayerCharacter` 0)))
  (set `/Game/ThirdPerson/Blueprints/BP_ThirdPersonCharacter.MaxHealth` (+ (`/Game/ThirdPerson/Blueprints/BP_ThirdPersonCharacter.MaxHealth` _asbp_third_person_character) 10.0) _asbp_third_person_character))

(fn `UserConstructionScript`
  (`parent.UserConstructionScript`))