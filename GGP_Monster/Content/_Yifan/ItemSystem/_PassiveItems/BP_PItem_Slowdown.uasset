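; Passive item Blueprint that slows the game world while largely preserving the player character's speed.
; Each UpdatePassiveEffect call runs the parent logic, then cuts global time dilation by a tenth of its current value.
; It also raises the player BP_ThirdPersonCharacter's CustomTimeDilation by a tenth, nearly offsetting the slowdown.
; Both changes are relative to current values, so repeated updates compound.
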(event `self.UpdatePassiveEffect`
  (bind _returnvalue (`GameplayStatics.GetGlobalTimeDilation`))
  (bind _asbp_third_person_character (cast `/Game/ThirdPerson/Blueprints/BP_ThirdPersonCharacter` (`GameplayStatics.GetPlayerCharacter` 0) :!pure true))
  (bind _customtimedilation (`Actor.CustomTimeDilation` _asbp_third_person_character))
  (`parent.UpdatePassiveEffect`)
  (`GameplayStatics.SetGlobalTimeDilation` (- _returnvalue (/ _returnvalue 10.0)))
  (set `Actor.CustomTimeDilation` (+ (/ _customtimedilation 10.0) _customtimedilation) _asbp_third_person_character))

(fn `UserConstructionScript`
  (`parent.UserConstructionScript`))