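; Passive item Blueprint that increases the player's damage reduction.
; Its UpdatePassiveEffect event adds a fixed increment to DamageReductionMultiplier on the Instance game instance, so each call stacks additively with no clamp in this asset.
; The other events are disabled stubs, and the construction script only calls its parent.
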(event `self.UpdatePassiveEffect`
  (bind _asinstance (cast `/Game/Instance/Instance` (`GameplayStatics.GetGameInstance`) :!pure true))
  (set `/Game/Instance/Instance.DamageReductionMultiplier` (+ (`/Game/Instance/Instance.DamageReductionMultiplier` _asinstance) 0.25) _asinstance))

(fn `UserConstructionScript`
  (`parent.UserConstructionScript`))