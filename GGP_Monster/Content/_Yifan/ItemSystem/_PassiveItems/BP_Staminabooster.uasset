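; BP_Staminabooster is a passive item that raises the player's maximum stamina.
; When its passive effect updates, it runs the parent logic, casts player 0's character to BP_ThirdPersonCharacter and adds a fixed amount to MaxStamina.
; It then prints the new maximum and calls RegenStamina on the character.
; Each update adds to the current value, so repeated calls stack.
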(event `self.UpdatePassiveEffect`
  (`parent.UpdatePassiveEffect`)
  (bind _asbp_third_person_character (cast `/Game/ThirdPerson/Blueprints/BP_ThirdPersonCharacter` (`GameplayStatics.GetPlayerCharacter` 0)))
  (bind _output_get (set `/Game/ThirdPerson/Blueprints/BP_ThirdPersonCharacter.MaxStamina` (+ (`/Game/ThirdPerson/Blueprints/BP_ThirdPersonCharacter.MaxStamina` _asbp_third_person_character) 20.0) _asbp_third_person_character))
  (`KismetSystemLibrary.PrintString` (`KismetStringLibrary.Conv_DoubleToString` _output_get))
  (`/Game/ThirdPerson/Blueprints/BP_ThirdPersonCharacter.Regen stamina` _asbp_third_person_character))

(fn `UserConstructionScript`
  (`parent.UserConstructionScript`))