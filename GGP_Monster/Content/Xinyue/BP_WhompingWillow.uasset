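; Whomping Willow tree actor that swings at whatever enters its trigger box and hurts the player on contact.
; Box overlap stores the intruder's location and plays a timeline that tilts the actor's roll, with yaw taken from FacePlayer.
; FacePlayer's arcsine angle calculation toward that location is left unconnected.
; Sphere overlap with the player plays a 2D sound created at BeginPlay, applies damage and adds a Niagara effect.
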(event `self.ReceiveBeginPlay`
  ;[1 1 1] Comment
  (set `self.OriginRotation` (`SceneComponent.K2_GetComponentRotation` (`self.DefaultSceneRoot`)))
  (set `self.Treet` (`SceneComponent.K2_GetComponentLocation` (`self.DefaultSceneRoot`)))
  (bind _returnvalue (`GameplayStatics.CreateSound2D` "/Game/Xinyue/Sound/SlimeAttack_Cue.SlimeAttack_Cue" 1.0 1.0 0.0 null false false))
  (set `self.sound` _returnvalue))

(event `self.Box.OnComponentBeginOverlap`
  (params (OverlappedComponent :type "PrimitiveComponent Object Reference") (OtherActor :type "Actor Object Reference") (OtherComp :type "PrimitiveComponent Object Reference") (OtherBodyIndex :type Integer) (bFromSweep :type Boolean) (SweepResult :type "HitResult Structure (by ref)"))
  (bind _player_x (`KismetMathLibrary.BreakVector` (`self.Player`)))
  (bind _treet_x (`KismetMathLibrary.BreakVector` (`self.Treet`)))
  (bind (_originrotation_roll _originrotation_pitch) (`KismetMathLibrary.BreakRotator` (`self.OriginRotation`)))
  ;[1 1 1] Comment
  (set `self.Player` (`SceneComponent.K2_GetComponentLocation` (`Actor.RootComponent` OtherActor)))
  (`|ExecutionSequence`
    (:`then_0`
      (bind (_direction _boxingplayer) (`Timeline|BoxingPlayer` :!via `PlayFromStart`)
        (:`Update`
          (`self.K2_SetActorRotation` (`KismetMathLibrary.MakeRotator` (`KismetMathLibrary.Lerp` 0.0 60.0 _boxingplayer) _originrotation_pitch (`KismetMathLibrary.DegAsin` (/ (- _treet_x _player_x) (`KismetMathLibrary.VSize` (- (`self.Treet`) (`self.Player`))))))))))))

(event `self.Sphere.OnComponentBeginOverlap`
  (params (OverlappedComponent :type "PrimitiveComponent Object Reference") (OtherActor :type "Actor Object Reference") (OtherComp :type "PrimitiveComponent Object Reference") (OtherBodyIndex :type Integer) (bFromSweep :type Boolean) (SweepResult :type "HitResult Structure (by ref)"))
  (bind _returnvalue (`SceneComponent.GetRelativeTransform` (`self.Sphere`)))
  (if (== OtherActor (`GameplayStatics.GetPlayerCharacter` 0))
    (set `self.Other Actor` OtherActor)
    (`|ExecutionSequence`
      (:`then_0`
        (`AudioComponent.Play` (`self.sound`) 0.0))
      (:`then_1`
        (`GameplayStatics.ApplyDamage` (`self.Other Actor`) (`self.Base Damage`) null self))
      (:`then_2`
        (`AddComponent|NODE_AddNiagaraComponent-0` :`RelativeTransform` (`KismetMathLibrary.MakeTransform` (`KismetMathLibrary.MakeVector` (- (.x (.location _returnvalue)) 50.0) (- (.y (.location _returnvalue)) 50.0) (- (.z (.location _returnvalue)) 100.0)) (.rotation _returnvalue) (.scale _returnvalue)))))))

(fn `UserConstructionScript`)