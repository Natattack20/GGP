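; BP_CarExhaust is a car exhaust hazard actor that damages the third-person player character.
; On BeginPlay it spawns a BP_CarExhaust1 actor at its Arrow component's transform.
; Each Tick it runs a box overlap sized to the StaticMesh bounds at the mesh's location, filtered to BP_ThirdPersonCharacter pawns.
; Every overlapping character takes CarExhaustDamage on each frame, so damage scales with frame rate.
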(event `self.ReceiveBeginPlay`
  ;[1 1 1] SpawnExhaust
  (`|SpawnActorFromClass` "/Game/Xinyue/BP_CarExhaust1.BP_CarExhaust1_C" (`SceneComponent.K2_GetComponentToWorld` (`self.Arrow`)) "AlwaysSpawn" "MultiplyWithRoot" null null))

(event `self.ReceiveTick`
  (params (DeltaSeconds :type "Float (single-precision)"))
  (bind _staticmesh (`self.StaticMesh`))
  ;[1 1 1] AttackPlayer
  (bind _outactors (`KismetSystemLibrary.BoxOverlapActors` (`SceneComponent.K2_GetComponentLocation` _staticmesh) (`.BoxExtent` (`KismetSystemLibrary.GetComponentBounds` _staticmesh)) (`|MakeArray` "ObjectTypeQuery3" :!type "EObjectTypeQuery Enum") "/Game/ThirdPerson/Blueprints/BP_ThirdPersonCharacter.BP_ThirdPersonCharacter_C" (`|MakeArray` self :!type "Actor Object Reference")))
  (for _array_element _outactors
    (`GameplayStatics.ApplyDamage` _array_element (`self.CarExhaustDamage`) null self)))

(fn `UserConstructionScript`)