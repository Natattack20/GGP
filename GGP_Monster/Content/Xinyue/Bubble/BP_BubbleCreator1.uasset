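; Bubble emitter actor that repeatedly spawns BP_Bubble actors at its ProjectilePos component.
; Tick calls SpawnBubble whenever none of the three tracked bubble references is valid.
; SpawnBubble plays a bubble sound at the mesh, then spawns three short-lived bubbles separated by BubblingBreakTime delays, storing each reference.
; A note on the delays says the break time must exceed the bubble duration.
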(event `self.ReceiveBeginPlay`)

(event `self.ReceiveTick`
  (params (DeltaSeconds :type "Float (single-precision)"))
  (`/Engine/EditorBlueprintResources/StandardMacros.IsValid` (`self.Bubble1`)
    (:`Is Not Valid`
      (`/Engine/EditorBlueprintResources/StandardMacros.IsValid` (`self.Bubble2`)
        (:`Is Not Valid`
          (`/Engine/EditorBlueprintResources/StandardMacros.IsValid` (`self.Bubble3`)
            (:`Is Not Valid`
              (`self.SpawnBubble`))))))))

(event `SpawnBubble`
  ;[1 1 1] Comment
  (`GameplayStatics.PlaySoundAtLocation` "/Game/Xinyue/Bubble/Sound/Bubble_Cue.Bubble_Cue" (`SceneComponent.K2_GetComponentLocation` (`self.StaticMesh`)) (struct) 1.0 1.0 0.0 null null null null)
  (bind _returnvalue (`|SpawnActorFromClass` "/Game/Xinyue/Bubble/BP_Bubble.BP_Bubble_C" (`SceneComponent.K2_GetComponentToWorld` (`self.ProjectilePos`)) "AlwaysSpawn" "MultiplyWithRoot" null null))
  (`self.SetLifeSpan` _returnvalue 6.1)
  (set `self.Bubble1` _returnvalue)
  (`KismetSystemLibrary.Delay` (`self.BubblingBreakTime`))
  (bind _returnvalue_2 (`|SpawnActorFromClass` "/Game/Xinyue/Bubble/BP_Bubble.BP_Bubble_C" (`SceneComponent.K2_GetComponentToWorld` (`self.ProjectilePos`)) "AlwaysSpawn" "MultiplyWithRoot" null null))
  (`self.SetLifeSpan` _returnvalue_2 6.1)
  (set `self.Bubble2` _returnvalue_2)
  (`KismetSystemLibrary.Delay` (`self.BubblingBreakTime`))
  (bind _returnvalue_3 (`|SpawnActorFromClass` "/Game/Xinyue/Bubble/BP_Bubble.BP_Bubble_C" (`SceneComponent.K2_GetComponentToWorld` (`self.ProjectilePos`)) "AlwaysSpawn" "MultiplyWithRoot" null null))
  (`self.SetLifeSpan` _returnvalue_3 6.1)
  (set `self.Bubble3` _returnvalue_3))

(fn `UserConstructionScript`)