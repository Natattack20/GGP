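; Hydrant actor that continuously emits water by spawning short-lived water actors at its Arrow component.
; Tick checks the stored Water and Water1 references and calls SpawnWater once neither is valid.
; SpawnWater creates one BP_HydrantWater and one BP_HydrantWater1 at the Arrow's world transform, gives each a brief lifespan and stores them, so their expiry drives the repeating cycle.
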(event `self.ReceiveTick`
  (params (DeltaSeconds :type "Float (single-precision)"))
  (`/Engine/EditorBlueprintResources/StandardMacros.IsValid` (`self.Water`)
    (:`Is Not Valid`
      (`/Engine/EditorBlueprintResources/StandardMacros.IsValid` (`self.water1`)
        (:`Is Not Valid`
          (`self.SpawnWater`))))))

(event `SpawnWater`
  (`|ExecutionSequence`
    (:`then_0`
      (bind _returnvalue (`|SpawnActorFromClass` "/Game/Xinyue/SpawnActor/BP_HydrantWater.BP_HydrantWater_C" (`SceneComponent.K2_GetComponentToWorld` (`self.Arrow`)) "AlwaysSpawn" "MultiplyWithRoot" null null))
      (`self.SetLifeSpan` _returnvalue 1.5)
      (set `self.Water` _returnvalue))
    (:`then_1`
      (bind _returnvalue_2 (`|SpawnActorFromClass` "/Game/Xinyue/SpawnActor/BP_HydrantWater1.BP_HydrantWater1_C" (`SceneComponent.K2_GetComponentToWorld` (`self.Arrow`)) "AlwaysSpawn" "MultiplyWithRoot" null null))
      (`self.SetLifeSpan` _returnvalue_2 1.5)
      (set `self.water1` _returnvalue_2))))

(fn `UserConstructionScript`)