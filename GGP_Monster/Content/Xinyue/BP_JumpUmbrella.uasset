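; Umbrella jump pad that bounces the third-person character along its Arrow component's forward direction.
; On box overlap, a timeline animates the actor's Z scale between 0.7 and 1.0 while a 2D umbrella sound, created at BeginPlay, plays.
; After a short delay, the character jumps and is then launched at Speed, with a DoOnce that resets after launch to block repeated triggers.
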(event `self.ReceiveBeginPlay`
  ;[1 1 1] Comment
  (set `self.Origin` (`self.GetActorScale3D`))
  (bind _returnvalue (`GameplayStatics.CreateSound2D` "/Game/Xinyue/Sound/Umbrella_Cue.Umbrella_Cue" 1.0 1.0 0.0 null false false))
  (set `self.Sound` _returnvalue))

(event `self.Box.OnComponentBeginOverlap`
  (params (OverlappedComponent :type "PrimitiveComponent Object Reference") (OtherActor :type "Actor Object Reference") (OtherComp :type "PrimitiveComponent Object Reference") (OtherBodyIndex :type Integer) (bFromSweep :type Boolean) (SweepResult :type "HitResult Structure (by ref)"))
  (bind (_origin_x _origin_y) (`KismetMathLibrary.BreakVector` (`self.Origin`)))
  ;[1 1 1] Comment
  (bind _asbp_third_person_character (cast `/Game/ThirdPerson/Blueprints/BP_ThirdPersonCharacter` OtherActor))
  (`|ExecutionSequence`
    (:`then_0`
      (bind (_direction _jump) (`Timeline|Umbrella` :!via `PlayFromStart`)
        (:`Update`
          (`self.SetActorScale3D` (`KismetMathLibrary.MakeVector` _origin_x _origin_y (`KismetMathLibrary.Lerp` 0.7 1.0 _jump))))))
    (:`then_1`
      (`AudioComponent.Play` (`self.Sound`) 0.1))
    (:`then_2`
      (`KismetSystemLibrary.Delay` 0.4)
      (`/Engine/EditorBlueprintResources/StandardMacros.DoOnce` false :!label _label
        (:`Completed`
          (`Character.Jump` _asbp_third_person_character)
          (`KismetSystemLibrary.Delay` 0.2)
          (`Character.LaunchCharacter` _asbp_third_person_character (* (`SceneComponent.GetForwardVector` (`self.Arrow`)) (`self.Speed`)) false false)
          (goto _label :!via `Reset`))))))

(fn `UserConstructionScript`)