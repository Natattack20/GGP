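; Car exhaust hazard actor that damages the player character on contact with its static mesh.
; On BeginPlay it spawns a second exhaust actor at its Arrow's transform and creates a persistent 2D smog sound.
; When the third-person character overlaps the mesh, it plays that sound, applies exhaust damage once and adds a Niagara effect, which it destroys after a short delay.
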(event `self.ReceiveBeginPlay`
  ;[1 1 1] SpawnExhaust
  (bind _returnvalue (`|SpawnActorFromClass` "/Game/Xinyue/SpawnActor/BP_CarExhaust1.BP_CarExhaust1_C" (`SceneComponent.K2_GetComponentToWorld` (`self.Arrow`)) "AlwaysSpawn" "MultiplyWithRoot" null null))
  (set `self.Exhaust2` _returnvalue)
  (bind _returnvalue_2 (`GameplayStatics.CreateSound2D` "/Game/Xinyue/Sound/CarSmog_Cue.CarSmog_Cue" 1.0 1.0 0.0 null false false))
  (set `self.CarDamage` _returnvalue_2))

(event `self.StaticMesh.OnComponentBeginOverlap`
  (params (OverlappedComponent :type "PrimitiveComponent Object Reference") (OtherActor :type "Actor Object Reference") (OtherComp :type "PrimitiveComponent Object Reference") (OtherBodyIndex :type Integer) (bFromSweep :type Boolean) (SweepResult :type "HitResult Structure (by ref)"))
  ;[1 1 1] AttackPlayer
  (bind _asbp_third_person_character (cast `/Game/ThirdPerson/Blueprints/BP_ThirdPersonCharacter` OtherActor))
  (`AudioComponent.Play` (`self.CarDamage`) 0.0)
  (`GameplayStatics.ApplyDamage` _asbp_third_person_character (`self.CarExhaustDamage`) null self)
  (bind _returnvalue (`AddComponent|NODE_AddNiagaraComponent-0` :`RelativeTransform` (`SceneComponent.GetRelativeTransform` (`self.StaticMesh`))))
  (`KismetSystemLibrary.Delay` 1.0)
  (`/Engine/EditorBlueprintResources/StandardMacros.IsValid` _returnvalue
    (:`Is Valid`
      (`ActorComponent.K2_DestroyComponent` _returnvalue))))

(fn `UserConstructionScript`)