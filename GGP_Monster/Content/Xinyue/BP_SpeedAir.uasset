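; BP_SpeedAir is a two-way boost actor that launches the third-person character along or against its Arrow, depending on the box entered.
; ABox and BBox set IsA/IsB flags so the opposite box skips its launch.
; Each launch replaces the Niagara effect on the player's mesh, removing it after a delay.
; Leaving CBox plays a trumpet sound and clears the active flag.
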(event `self.ReceiveBeginPlay`
  (bind _returnvalue (`GameplayStatics.CreateSound2D` "/Game/Xinyue/Sound/Trumpet1_Cue.Trumpet1_Cue" 1.0 1.0 0.0 null false false))
  (set `self.Sound` _returnvalue))

(event `self.ABox.OnComponentBeginOverlap`
  (params (OverlappedComponent :type "PrimitiveComponent Object Reference") (OtherActor :type "Actor Object Reference") (OtherComp :type "PrimitiveComponent Object Reference") (OtherBodyIndex :type Integer) (bFromSweep :type Boolean) (SweepResult :type "HitResult Structure (by ref)"))
  (bind _returnvalue (`GameplayStatics.GetPlayerCharacter` 0))
  (bind _vef1 (`self.VEF1`))
  (bind _returnvalue_2 (`SceneComponent.K2_GetComponentRotation` (`Actor.RootComponent` _returnvalue)))
  ;[1 1 1] Comment
  (cast `/Game/ThirdPerson/Blueprints/BP_ThirdPersonCharacter` OtherActor)
  (if (`self.IsB`)
    (set `self.IsA` false)
    (else
      (set `self.IsA` true)
      (`/Engine/EditorBlueprintResources/StandardMacros.IsValid` _vef1
        (:`Is Valid`
          (`ActorComponent.K2_DestroyComponent` _vef1))
        (:`Is Not Valid`
          _))
      (`/Engine/EditorBlueprintResources/StandardMacros.DoOnce` false :!label _label
        (:`Completed`
          (bind _returnvalue_3 (`AddComponent|NODE_AddNiagaraComponent-1`))
          (bind _output_get (set `self.VEF1` _returnvalue_3))
          (`SceneComponent.K2_SetWorldRotation` _output_get _returnvalue_2 false false)
          (`/Engine/EditorBlueprintResources/StandardMacros.IsValid` _output_get
            (:`Is Valid`
              (`SceneComponent.K2_AttachToComponent` _output_get (`Character.Mesh` _returnvalue) "None" "SnapToTarget" "KeepWorld" "KeepRelative" true)
              (`SceneComponent.K2_SetWorldRotation` _output_get _returnvalue_2 false false)
              (`|ExecutionSequence`
                (:`then_0`
                  (`Character.LaunchCharacter` _returnvalue (* (`SceneComponent.GetForwardVector` (`self.Arrow`)) (* (`self.SPEED`) -1.0)) false false)
                  (goto _label :!via `Reset`))
                (:`then_1`
                  (`KismetSystemLibrary.Delay` 3.0)
                  (`/Engine/EditorBlueprintResources/StandardMacros.IsValid` _output_get
                    (:`Is Valid`
                      (`ActorComponent.K2_DestroyComponent` _output_get))))))))))))

(event `self.ABox.OnComponentEndOverlap`
  (params (OverlappedComponent :type "PrimitiveComponent Object Reference") (OtherActor :type "Actor Object Reference") (OtherComp :type "PrimitiveComponent Object Reference") (OtherBodyIndex :type Integer))
  ;[1 1 1] Comment
  (cast `/Game/ThirdPerson/Blueprints/BP_ThirdPersonCharacter` OtherActor))

(event `self.BBox.OnComponentBeginOverlap`
  (params (OverlappedComponent :type "PrimitiveComponent Object Reference") (OtherActor :type "Actor Object Reference") (OtherComp :type "PrimitiveComponent Object Reference") (OtherBodyIndex :type Integer) (bFromSweep :type Boolean) (SweepResult :type "HitResult Structure (by ref)"))
  (bind _returnvalue (`GameplayStatics.GetPlayerCharacter` 0))
  (bind _vef1 (`self.VEF1`))
  (bind _returnvalue_2 (`SceneComponent.K2_GetComponentRotation` (`Actor.RootComponent` _returnvalue)))
  ;[1 1 1] Comment
  (cast `/Game/ThirdPerson/Blueprints/BP_ThirdPersonCharacter` OtherActor)
  (if (`self.IsA`)
    (set `self.IsB` false)
    (else
      (set `self.IsB` true)
      (`/Engine/EditorBlueprintResources/StandardMacros.IsValid` _vef1
        (:`Is Valid`
          (`ActorComponent.K2_DestroyComponent` _vef1))
        (:`Is Not Valid`
          _))
      (`/Engine/EditorBlueprintResources/StandardMacros.DoOnce` false :!label _label_2
        (:`Completed`
          (bind _returnvalue_3 (`AddComponent|NODE_AddNiagaraComponent-3`))
          (bind _output_get (set `self.VEF1` _returnvalue_3))
          (`SceneComponent.K2_SetWorldRotation` _output_get _returnvalue_2 false false)
          (`/Engine/EditorBlueprintResources/StandardMacros.IsValid` _output_get
            (:`Is Valid`
              (`SceneComponent.K2_AttachToComponent` _output_get (`Character.Mesh` _returnvalue) "None" "SnapToTarget" "KeepWorld" "KeepRelative" true)
              (`SceneComponent.K2_SetWorldRotation` _output_get _returnvalue_2 false false)
              (`|ExecutionSequence`
                (:`then_0`
                  (`Character.LaunchCharacter` _returnvalue (* (`SceneComponent.GetForwardVector` (`self.Arrow`)) (`self.SPEED`)) false false)
                  (goto _label_2 :!via `Reset`))
                (:`then_1`
                  (`KismetSystemLibrary.Delay` 3.0)
                  (`/Engine/EditorBlueprintResources/StandardMacros.IsValid` _output_get
                    (:`Is Valid`
                      (`ActorComponent.K2_DestroyComponent` _output_get))))))))))))

(event `self.BBox.OnComponentEndOverlap`
  (params (OverlappedComponent :type "PrimitiveComponent Object Reference") (OtherActor :type "Actor Object Reference") (OtherComp :type "PrimitiveComponent Object Reference") (OtherBodyIndex :type Integer))
  ;[1 1 1] Comment
  (cast `/Game/ThirdPerson/Blueprints/BP_ThirdPersonCharacter` OtherActor))

(event `self.CBox.OnComponentEndOverlap`
  (params (OverlappedComponent :type "PrimitiveComponent Object Reference") (OtherActor :type "Actor Object Reference") (OtherComp :type "PrimitiveComponent Object Reference") (OtherBodyIndex :type Integer))
  ;[1 1 1] Comment
  (cast `/Game/ThirdPerson/Blueprints/BP_ThirdPersonCharacter` OtherActor)
  (`AudioComponent.Play` (`self.Sound`) 0.0)
  (if (`self.IsA`)
    (set `self.IsA` false)
    (elif (`self.IsB`)
      (set `self.IsB` false))))

(event `self.CBox.OnComponentBeginOverlap`
  (params (OverlappedComponent :type "PrimitiveComponent Object Reference") (OtherActor :type "Actor Object Reference") (OtherComp :type "PrimitiveComponent Object Reference") (OtherBodyIndex :type Integer) (bFromSweep :type Boolean) (SweepResult :type "HitResult Structure (by ref)"))
  ;[1 1 1] Comment
  (cast `/Game/ThirdPerson/Blueprints/BP_ThirdPersonCharacter` OtherActor))

(fn `UserConstructionScript`)